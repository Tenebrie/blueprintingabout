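; Base actor component for timed buffs in the buff system, counting down its duration and removing itself on expiry.
; Tick subtracts delta time from Duration and destroys the component once it drops below zero.
; Adding stacks updates StackCount and resets Duration to BaseDuration.
; It also exposes a neutral walk speed scalar and a DestroySelf function for direct removal.
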(event EventBeginPlay)

(event EventTick
  (params (DeltaSeconds :type Float%20%28single-precision%29))
  (bind _output_get (Variables|Default|SetDuration (- (Variables|Default|GetDuration) DeltaSeconds)))
  (if (< _output_get 0.0)
    (Components|DestroyComponent)))

(fn OnExtraStacksAdded
  (params (StackCount :type Integer))
  (Variables|Default|SetStackCount (+ StackCount (Variables|Default|GetStackCount)))
  (CallFunction|RefreshDuration))

(fn RefreshDuration
  (Variables|Default|SetDuration (Variables|Default|GetBaseDuration)))

(fn GetWalkSpeedScalar
  (return 1.0))

(fn DestroySelf
  (Components|DestroyComponent))