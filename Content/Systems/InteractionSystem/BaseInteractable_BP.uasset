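; Base interactable Blueprint for world items the player can pick up.
; The construction script scans the ItemInfo data table and copies the row whose ItemID matches the chosen ItemName enum into ItemInfo.
; On Interact, it passes ItemInfo to BP_Player's PickupItem and destroys itself.
; It reports itself as single-use.
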(event EventInteract
  (bind _asplayer_bp (Utilities|Casting|CastToBP_Player (Game|GetPlayerCharacter 0)))
  (Default|PickupItem _asplayer_bp (Variables|Default|GetItemInfo))
  (Actor|DestroyActor))

(fn ConstructionScript
  (bind _outrownames (DataTable|GetDataTableRowNames "/Game/Systems/InteractionSystem/ItemInfo_DT.ItemInfo_DT"))
  (bind _array_element (Utilities|Array|ForEachLoopwithBreak _outrownames)
    (:LoopBody
      (bind _returnvalue (Utilities|GetDataTableRow "/Game/Systems/InteractionSystem/ItemInfo_DT.ItemInfo_DT" _array_element)
        (:then
          (if (== (Utilities|Name|EnumtoName (.ItemID (Utilities|Struct|BreakItemInfo_S _returnvalue))) (Utilities|Name|EnumtoName (Variables|Default|GetItemName)))
            (Variables|Default|SetItemInfo _returnvalue)))))))

(fn IsSingleUse
  (return true))