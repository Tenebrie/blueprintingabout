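; Actor component that drives a dissolve effect on a target mesh and can remove its owning actor afterwards.
; On BeginPlay it creates a dynamic material instance for the chosen material slot of the target mesh.
; Each tick it raises the DissolveAmount scalar parameter by DissolveSpeed scaled by delta time, with no clamp.
; If CleanUpActor is set, it destroys the owner once that amount passes a hardcoded threshold.
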(event EventBeginPlay
  (bind _returnvalue (Rendering|Material|CreateDynamicMaterialInstance (Variables|Default|GetTargetMesh) (Variables|Default|GetTargetMaterialIndex) (Rendering|Material|GetMaterial (Variables|Default|GetTargetMesh) (Variables|Default|GetTargetMaterialIndex)) "None" :!class /Script/Engine.PrimitiveComponent))
  (Variables|Default|SetMaterial _returnvalue))

(event EventTick
  (params (DeltaSeconds :type Float%20%28single-precision%29))
  (bind _returnvalue (Rendering|Material|GetScalarParameterValue (Variables|Default|GetMaterial) "DissolveAmount" :!class /Script/Engine.MaterialInstanceDynamic))
  (Rendering|Material|SetScalarParameterValue (Variables|Default|GetMaterial) "DissolveAmount" (+ _returnvalue (* DeltaSeconds (Variables|Default|GetDissolveSpeed))) :!class /Script/Engine.MaterialInstanceDynamic)
  (if (and (> (+ _returnvalue (* DeltaSeconds (Variables|Default|GetDissolveSpeed))) 5.0) (Variables|Default|GetCleanUpActor))
    (Actor|DestroyActor (Components|GetOwner))))