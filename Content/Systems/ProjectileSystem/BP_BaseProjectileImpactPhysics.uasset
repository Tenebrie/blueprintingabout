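; BP_BaseProjectileImpactPhysics is a one-shot Chaos field actor that applies destruction physics at a projectile impact point.
; On BeginPlay, a radial falloff field centred on its Sphere applies external cluster strain to fracture geometry collections.
; A radial vector linear force, culled outside a smaller radius by a second falloff, then pushes pieces outward.
; The actor destroys itself immediately after both fields are applied.
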(event EventBeginPlay
  (Class|FieldSystemComponent|ApplyPhysicsField (Variables|Field|GetFieldSystemComponent) true "Field_ExternalClusterStrain" 0 (Field|SetRadialFalloff (Variables|Default|GetRadialFalloff) 1e+07 0.0 1.0 0.0 2.5e+02 (Transformation|GetWorldLocation (Variables|Default|GetSphere)) "Field_Falloff_Linear"))
  (Class|FieldSystemComponent|ApplyPhysicsField (Variables|Field|GetFieldSystemComponent) true "Field_LinearForce" 0 (Field|SetCullingField (Variables|Default|GetCullingField) (Field|SetRadialFalloff (Variables|Default|GetRadialFalloff) 1e+07 0.0 1.0 0.0 1e+02 (Transformation|GetWorldLocation (Variables|Default|GetSphere)) "Field_Falloff_Linear") (Field|SetRadialVector (Variables|Default|GetRadialVector) 1e+07 (Transformation|GetWorldLocation (Variables|Default|GetSphere))) "Field_Culling_Outside"))
  (Actor|DestroyActor))

(fn ConstructionScript)