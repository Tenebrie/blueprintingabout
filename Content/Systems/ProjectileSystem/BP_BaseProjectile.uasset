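; Base projectile actor that moves forward by swept offsets each tick until it hits something or its lifetime expires.
; On overlap it damages enemy units by alignment and applies impulses to them or movable props, blending travel and target directions.
; A state enum drives movement, impact Niagara with fading light, and delayed cleanup.
; GetDamage is a placeholder returning zero, and OnTargetHit and OnStateChanged are empty hooks.
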(event OnComponentBeginOverlap(Coll)
  (params (OverlappedComponent :type Primitive%20Component%20Object%20Reference) (OtherActor :type Actor%20Object%20Reference) (OtherComp :type Primitive%20Component%20Object%20Reference) (OtherBodyIndex :type Integer) (bFromSweep :type Boolean) (SweepResult :type Hit%20Result%20Structure%20%28by%20ref%29))
  (bind _returnvalue (Math|Float|Absolute(Float) 1e+04))
  (Variables|SingleUse|SetImpactTargetActor OtherActor)
  (Variables|SingleUse|SetImpactTargetComponent OtherComp)
  (if (Private|IsActorValidImpactTarget (Variables|SingleUse|GetImpactTargetActor))
    (if (.IsUnit (CallFunction|GetActorUnitStats (Variables|SingleUse|GetImpactTargetActor)))
      (Variables|SingleUse|SetImpactTargetUnitStats (.UnitStats (CallFunction|GetActorUnitStats (Variables|SingleUse|GetImpactTargetActor))))
      (if (CallFunction|IsEnemy (Default|GetAlignment (Variables|SingleUse|GetImpactTargetUnitStats)) (Variables|Provided|GetProjectileAlignment))
        (bind (_forcemesh _forcebonename _forcemultiplier) (Default|DealDamage (Variables|SingleUse|GetImpactTargetUnitStats) (CallFunction|GetPlayerProjectileDI self (Variables|SingleUse|GetImpactTargetActor))))
        (CallFunction|OnTargetHit (Variables|SingleUse|GetImpactTargetActor))
        (if (Utilities|IsValid _forcemesh)
          (Variables|SingleUse|SetImpactTargetComponent _forcemesh))
        (Variables|SingleUse|SetImpactTargetBoneName _forcebonename)
        (Variables|SingleUse|SetImpactForceMultiplier _forcemultiplier)
        (Private|DestroyProjectile :!label _label)
        (Physics|AddImpulseatLocation (Variables|SingleUse|GetImpactTargetComponent) (* (* (Math|Vector|MakeVector _returnvalue _returnvalue _returnvalue) (Private|GetImpactForceVector (Variables|SingleUse|GetImpactTargetComponent))) (Variables|SingleUse|GetImpactForceMultiplier)) (Transformation|GetActorLocation) (Variables|SingleUse|GetImpactTargetBoneName)))
      (else
        (Variables|SingleUse|SetImpactForceMultiplier 1.0)
        (if (Private|IsComponentMovable (Variables|SingleUse|GetImpactTargetComponent))
          (goto _label)
          (else
            (Private|DestroyProjectile)))))))

(event Custom|OnCleanup
  (Utilities|FlowControl|Delay 3.0)
  (Variables|Default|SetProjectileState "NewEnumerator3")
  (Collision|SetActorEnableCollision self false)
  (Utilities|FlowControl|Delay 3.0)
  (Actor|DestroyActor))

(event Custom|OnStateChanged
  (params (State :type E_ProjectileState%20Enum :default "NewEnumerator0")))

(event EventTick
  (params (DeltaSeconds :type Float%20%28single-precision%29))
  (Variables|SingleUse|SetDeltaSeconds DeltaSeconds)
  (Private|TickProjectileLifetime)
  (Private|TickProjectileMovement)
  (Private|TickProjectileDecay)
  (Private|TickProjectileCleanup))

(event Custom|OnTargetHit
  (params (Target :type Actor%20Object%20Reference)))

(fn ConstructionScript)

(fn GetImpactForceVector
  (params (ImpactTargetComponent :type Primitive%20Component%20Object%20Reference))
  (return (Math|Vector|Normalize (+ (Math|Vector|Normalize (Math|Vector|GetForwardVector (Transformation|GetActorRotation))) (Math|Vector|GetUnitDirection(Vector) (Transformation|GetActorLocation) (Transformation|GetWorldLocation ImpactTargetComponent))))))

(fn DestroyProjectile
  (if (not (Variables|Default|GetProjectileDestroyed))
    (Variables|Default|SetProjectileDestroyed true)
    (CallFunction|UpdateProjectileStateandNotify "NewEnumerator2")
    (Class|NiagaraComponent|SetVariableBool (Actor|GetComponentsByClass "/Script/Niagara.NiagaraComponent") "IsEnabled" false)
    (Niagara|SpawnSystematLocation (Variables|ProjectileProperties|GetProjectileImpactNiagaraEffect) (Transformation|GetActorLocation) (Transformation|GetActorRotation))
    (CallFunction|OnCleanup)))

(fn TickProjectileLifetime
  (bind _output_get (Variables|Default|SetProjectileCurrentLifetime (+ (Variables|Default|GetProjectileCurrentLifetime) (Variables|SingleUse|GetDeltaSeconds))))
  (if (>= _output_get (Variables|ProjectileProperties|GetProjectileMaxLifetime))
    (Private|DestroyProjectile)))

(fn TickProjectileMovement
  (if (Utilities|Enum|Equal(Enum) (Variables|Default|GetProjectileState) "NewEnumerator1")
    (Transformation|AddActorLocalOffset (* (Math|Vector|MakeVector (Variables|ProjectileProperties|GetProjectileSpeed) 0.0 0.0) (Variables|SingleUse|GetDeltaSeconds)) true false)))

(fn TickProjectileDecay
  (bind _pointlight (Variables|Default|GetPointLight))
  (bind _pointlight_2 (Variables|Default|GetPointLight))
  (if (Utilities|Enum|Equal(Enum) (Variables|Default|GetProjectileState) "NewEnumerator2")
    (Utilities|FlowControl|Sequence
      (:then_0
        (Rendering|Lighting|SetAttenuationRadius _pointlight_2 (- (Variables|/Script/Engine.LocalLightComponent|GetAttenuationRadius _pointlight_2) (* (Variables|SingleUse|GetDeltaSeconds) 5e+03))))
      (:then_1
        (Rendering|Components|Light|SetIntensity _pointlight (- (Variables|/Script/Engine.LightComponentBase|GetIntensity _pointlight) (* (Variables|SingleUse|GetDeltaSeconds) 2.5e+04)))))))

(fn TickProjectileCleanup
  (if (Utilities|Enum|Equal(Enum) (Variables|Default|GetProjectileState) "NewEnumerator3")
    _))

(fn IsActorValidImpactTarget
  (params (Actor :type Actor%20Object%20Reference))
  (bind _projectilestate (Variables|Default|GetProjectileState))
  (return (Math|Boolean|ANDBoolean (or (== (Utilities|GetClass Actor) "/Script/Engine.StaticMeshActor") (Actor|ActorHasTag Actor (GameplayTags|GetTagName (GameplayTags|MakeLiteralGameplayTag "(TagName=\"is_unit\")")))) (Utilities|Enum|NotEqual(Enum) _projectilestate "NewEnumerator2") (Utilities|Enum|NotEqual(Enum) _projectilestate "NewEnumerator3"))))

(fn IsComponentMovable
  (params (Component :type Scene%20Component%20Object%20Reference))
  (return (Utilities|Enum|Equal(Enum) (Variables|/Script/Engine.SceneComponent|GetMobility Component) "Movable")))

(fn UpdateProjectileStateandNotify
  (params (Desired%20State :type E_ProjectileState%20Enum :default "NewEnumerator0"))
  (LocalVariables|SetNewState Desired%20State)
  (LocalVariables|SetPreviousState (Variables|Default|GetProjectileState))
  (Utilities|FlowControl|Sequence
    (:then_0
      (if (and (Utilities|Enum|Equal(Enum) (LocalVariables|GetNewState) "NewEnumerator1") (Variables|Default|GetProjectileDestroyed))
        (LocalVariables|SetNewState "NewEnumerator2")))
    (:then_1
      (bind _output_get (Variables|Default|SetProjectileState (LocalVariables|GetNewState)))
      (if (Utilities|Enum|NotEqual(Enum) (LocalVariables|GetNewState) (LocalVariables|GetPreviousState))
        (CallFunction|OnStateChanged _output_get)))))

(fn GetDamage
  (params (DamageImpactTarget :type Actor%20Object%20Reference))
  (Development|PrintString "This projectile don't have get damage function implemented")
  (return 0.0 "NewEnumerator0" 1.0))