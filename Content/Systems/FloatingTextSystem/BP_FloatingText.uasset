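; Floating text actor that shows a configurable message through a widget component, drifts away and fades out.
; The construction script copies the displayed text into the UI_FloatingTextInstance widget; BeginPlay passes it text, size, color and fade timing.
; BeginPlay also picks a random horizontal drift with constant upward motion, applied each Tick as a local offset.
; The actor destroys itself shortly after the fade completes.
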(event EventBeginPlay
  (Variables|Default|SetMovementOffsetVector (Math|Vector|MakeVector (Math|Random|RandomFloatinRange -1.0 1.0) (Math|Random|RandomFloatinRange -1.0 1.0) 1.0))
  (bind _asui_floating_text_instance (Utilities|Casting|CastToUI_FloatingTextInstance (UserInterface|GetWidget (Variables|Default|GetWidget))))
  (Default|SetProperties _asui_floating_text_instance (Variables|Default|GetDisplayedText) (Variables|Default|GetFontSizeScalar) (Variables|Default|GetTextColor) (Variables|Default|GetFadeOutAt) (Variables|Default|GetFadeOutDuration))
  (Utilities|FlowControl|Delay (+ (Variables|Default|GetFadeOutAt) (Variables|Default|GetFadeOutDuration) 0.1))
  (Actor|DestroyActor))

(event EventTick
  (params (DeltaSeconds :type Float%20%28single-precision%29))
  (Transformation|AddActorLocalOffset (* "100.000000,100.000000,150.000000" DeltaSeconds (Variables|Default|GetMovementOffsetVector)) false false))

(fn ConstructionScript
  (bind _asui_floating_text_instance (Utilities|Casting|CastToUI_FloatingTextInstance (UserInterface|GetWidget (Variables|Default|GetWidget))))
  (Variables|/Game/Systems/FloatingTextSystem/UI_FloatingTextInstance.UI_FloatingTextInstance_C|SetText _asui_floating_text_instance (Variables|Default|GetDisplayedText)))