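; Base interactable actor for item pickups that hands its item data to the player and then removes itself from the world.
; The Construction Script scans every row of ItemInfo_DT and caches the one whose ItemID enum name matches ItemName as ItemInfo.
; Interact casts player character 0 to BP_Player, calls PickupItem with that data and destroys the actor.
; IsSingleUse always reports true.
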(event EventInteract
  (bind _asbp_player (Utilities|Casting|CastToBP_Player (Game|GetPlayerCharacter 0)))
  (Default|PickupItem _asbp_player (Variables|Default|GetItemInfo))
  (Actor|DestroyActor))

(fn ConstructionScript
  (bind _outrownames (DataTable|GetDataTableRowNames "/Game/Systems/ItemPickupSystem/ItemInfo_DT.ItemInfo_DT"))
  (bind _array_element (Utilities|Array|ForEachLoopwithBreak _outrownames)
    (:LoopBody
      (bind _returnvalue (Utilities|GetDataTableRow "/Game/Systems/ItemPickupSystem/ItemInfo_DT.ItemInfo_DT" _array_element)
        (:then
          (if (== (Utilities|Name|EnumtoName (.ItemID (Utilities|Struct|BreakItemInfo_S _returnvalue))) (Utilities|Name|EnumtoName (Variables|Default|GetItemName)))
            (Variables|Default|SetItemInfo _returnvalue)))))))

(fn IsSingleUse
  (return true))