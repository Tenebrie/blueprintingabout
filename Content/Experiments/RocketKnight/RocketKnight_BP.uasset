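; Experimental rocket knight Blueprint that propels a physics-driven knight body with a switchable engine.
; EnableEngine and DisableEngine set the engine flag and turn the EngineFX particle spawn rate on or off.
; While enabled, Tick applies a constant-magnitude force to KnightBody along ForwardBox's forward vector, so that component steers the thrust.
; BeginPlay zeroes the effect's spawn rate, and IsEngineEnabled exposes the flag.
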(event EventTick
  (params (DeltaSeconds :type Float%20%28single-precision%29))
  ;[1 1 1] Flying
  (if (Variables|Default|Get__IsEngineEnabled)
    (Physics|AddForce (Variables|Default|GetKnightBody) (* (Math|Vector|GetForwardVector (Transformation|GetWorldRotation (Variables|Default|GetForwardBox))) 2e+05) "None" false)))

(event EventBeginPlay
  ;[1 1 1] Enable/Disable
  (Niagara|SetNiagaraVariable(Float) (Variables|Default|GetEngine_FX) "SpawnRate" 0.0))

(event EventEnableEngine
  ;[1 1 1] Enable/Disable
  (Variables|Default|Set__IsEngineEnabled true)
  (Niagara|SetNiagaraVariable(Float) (Variables|Default|GetEngine_FX) "SpawnRate" 2.5e+03))

(event EventDisableEngine
  ;[1 1 1] Enable/Disable
  (Variables|Default|Set__IsEngineEnabled false)
  (Niagara|SetNiagaraVariable(Float) (Variables|Default|GetEngine_FX) "SpawnRate" 0.0))

(fn ConstructionScript)

(fn IsEngineEnabled
  (return (Variables|Default|Get__IsEngineEnabled)))