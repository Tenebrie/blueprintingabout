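; Player controller that creates the main UI, registers a hardcoded set of spells and slots with its inventory, and drives spell casting from input.
; Assigning a spell to a binding adds its controller component to the controlled pawn, replacing any previous one; clearing destroys it.
; Tick-driven gates cast while Primary, Secondary or Movement input is held; Movement uses the primary binding's spell in movement mode.
; CastSpell is an empty stub.
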(event Custom|OnTickPrimaryAction
  (bind _spellinputbindings (Variables|Default|GetSpellInputBindings))
  (bind (_value _returnvalue) (Utilities|Map|Find _spellinputbindings "NewEnumerator0"))
  (if _returnvalue
    (Utilities|FlowControl|Gate true
      (:Exit
        (Default|OnSpellCastasActive (.SpellControllerComponent (Utilities|Struct|BreakS_SpellInputBinding _value)))))))

(event Custom|OnTickSecondaryAction
  (bind _spellinputbindings (Variables|Default|GetSpellInputBindings))
  (bind (_value _returnvalue) (Utilities|Map|Find _spellinputbindings "NewEnumerator1"))
  (if _returnvalue
    (Utilities|FlowControl|Gate true
      (:Exit
        (Default|OnSpellCastasActive (.SpellControllerComponent (Utilities|Struct|BreakS_SpellInputBinding _value)))))))

(event Custom|OnTickMovementAction
  (bind _spellinputbindings (Variables|Default|GetSpellInputBindings))
  (bind (_value _returnvalue) (Utilities|Map|Find _spellinputbindings "NewEnumerator0"))
  (if _returnvalue
    (Utilities|FlowControl|Gate true
      (:Exit
        (Default|OnSpellCastasMovement (.SpellControllerComponent (Utilities|Struct|BreakS_SpellInputBinding _value)))))))

(event EventBeginPlay
  (bind _returnvalue (UserInterface|CreateWidget "/Game/Systems/UserInterface/UI_Main.UI_Main_C" self))
  (bind _output_get (Variables|Default|SetPlayerUIRef _returnvalue))
  (UserInterface|Viewport|AddtoViewport _output_get 0)
  (for _array_element (Utilities|Array|MakeArray (Utilities|Struct|MakeS_Spell "Fireball" "/Game/Abilities/Fireball/Icon_Fireball.Icon_Fireball" "/Game/Abilities/Fireball/BPC_FireballController.BPC_FireballController_C") (Utilities|Struct|MakeS_Spell "Rockball" "/Game/Abilities/Rockball/Icon_RockThrow.Icon_RockThrow" "/Game/Abilities/Rockball/BPC_RockThrowController.BPC_RockThrowController_C") (Utilities|Struct|MakeS_Spell "Lightningball" "/Game/Assets/Icons/potions/potion3.potion3" "/Game/Abilities/Fireball/BPC_FireballController.BPC_FireballController_C") (Utilities|Struct|MakeS_Spell "Football" "/Game/Assets/Icons/potions/potion24.potion24" "/Game/Abilities/Fireball/BPC_FireballController.BPC_FireballController_C"))
    (Default|RegisterSpell (Variables|/Game/Systems/UserInterface/UI_Main.UI_Main_C|GetInventoryComponent (Variables|Default|GetPlayerUIRef)) _array_element))
  (for _array_element_2 (Utilities|Array|MakeArray (Utilities|Struct|MakeS_SpellSlot "NewEnumerator0" false "(Name_6_4FA140DA4B20C7435275198BDFBC1EF9=\"\",Icon_11_5D3445D549293F6D1F29F5AA0FBB74A5=None,ControlComponentClass_8_CA0FF916438F5A106C180AAB7D59355E=None)") (Utilities|Struct|MakeS_SpellSlot "NewEnumerator1" false "(Name_6_4FA140DA4B20C7435275198BDFBC1EF9=\"\",Icon_11_5D3445D549293F6D1F29F5AA0FBB74A5=None,ControlComponentClass_8_CA0FF916438F5A106C180AAB7D59355E=None)") (Utilities|Struct|MakeS_SpellSlot "NewEnumerator2" false "(Name_6_4FA140DA4B20C7435275198BDFBC1EF9=\"\",Icon_11_5D3445D549293F6D1F29F5AA0FBB74A5=None,ControlComponentClass_8_CA0FF916438F5A106C180AAB7D59355E=None)"))
    (Default|RegisterSpellSlot (Variables|/Game/Systems/UserInterface/UI_Main.UI_Main_C|GetInventoryComponent (Variables|Default|GetPlayerUIRef)) _array_element_2)))

(event EventTick
  (params (DeltaSeconds :type Float%20%28single-precision%29))
  (Variables|Default|SetDeltaSeconds DeltaSeconds)
  (CallFunction|OnTickMovementAction)
  (CallFunction|OnTickPrimaryAction)
  (CallFunction|OnTickSecondaryAction))

(event Input|ActionEvents|InputActionPrimaryAction
  (params (Key :type Key%20Structure :default "None"))
  (:Pressed
    (Utilities|FlowControl|Gate true) ; enters at Open
  )
  (:Released
    (Utilities|FlowControl|Gate true) ; enters at Close
  ))

(event Input|ActionEvents|InputActionSecondaryAction
  (params (Key :type Key%20Structure :default "None"))
  (:Pressed
    (Utilities|FlowControl|Gate true) ; enters at Open
  )
  (:Released
    (Utilities|FlowControl|Gate true) ; enters at Close
  ))

(event Input|ActionEvents|InputActionMovementAction
  (params (Key :type Key%20Structure :default "None"))
  (:Pressed
    (Utilities|FlowControl|Gate true) ; enters at Open
  )
  (:Released
    (Utilities|FlowControl|Gate true) ; enters at Close
  ))

(fn ConstructionScript)

(fn AssignSpelltoBinding
  (params (Spell :type S%20Spell%20Structure) (Binding :type E_SpellSlotBinding%20Enum :default "NewEnumerator0"))
  (LocalVariables|SetSpellData Spell)
  (LocalVariables|SetSpellBinding Binding)
  (Utilities|FlowControl|Sequence
    (:then_0
      ;[1 1 1] Destroy Component If Old Binding Exists
      (if (.ReturnValue (Utilities|Map|Find (Variables|Default|GetSpellInputBindings) (LocalVariables|GetSpellBinding)))
        (Components|DestroyComponent (.SpellControllerComponent (Utilities|Struct|BreakS_SpellInputBinding (.Value (Utilities|Map|Find (Variables|Default|GetSpellInputBindings) (LocalVariables|GetSpellBinding))))))))
    (:then_1
      ;[1 1 1] Create New Binding
      (bind _returnvalue (Game|AddComponentbyClass (Pawn|GetControlledPawn) (.ControlComponentClass (Utilities|Struct|BreakS_Spell (LocalVariables|GetSpellData)))))
      (Utilities|Map|Add (Variables|Default|GetSpellInputBindings) (LocalVariables|GetSpellBinding) (Utilities|Struct|MakeS_SpellInputBinding (LocalVariables|GetSpellData) _returnvalue)))))

(fn CastSpell
  (params (Spell :type S%20Spell%20Structure)))

(fn ClearSpellBinding
  (params (Binding :type E_SpellSlotBinding%20Enum :default "NewEnumerator0"))
  (LocalVariables|SetSpellBinding Binding)
  (Utilities|FlowControl|Sequence
    (:then_0
      ;[1 1 1] Destroy Component If Old Binding Exists
      (if (.ReturnValue (Utilities|Map|Find (Variables|Default|GetSpellInputBindings) (LocalVariables|GetSpellBinding)))
        (Components|DestroyComponent (.SpellControllerComponent (Utilities|Struct|BreakS_SpellInputBinding (.Value (Utilities|Map|Find (Variables|Default|GetSpellInputBindings) (LocalVariables|GetSpellBinding))))))))
    (:then_1
      ;[1 1 1] Remove Old Binding
      (Utilities|Map|Remove (Variables|Default|GetSpellInputBindings) (LocalVariables|GetSpellBinding)))))