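; Base enemy character that tracks health and reacts to damage with physics-driven hit reactions and a death ragdoll.
; Non-lethal damage simulates bodies below the spine, and Tick fades their physics blend weight out over about a second.
; Lethal damage simulates the mesh and switches the bone to the hips.
; TakeDamage returns the mesh and bone for applying force, while GetHealth always returns zero.
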(event EventTick
  (params (DeltaSeconds :type Float%20%28single-precision%29))
  (if (> (Variables|Default|GetRagdollWeight) 0.0)
    (bind _output_get (Variables|Default|SetRagdollWeight (- (Variables|Default|GetRagdollWeight) DeltaSeconds)))
    (Class|SkeletalMeshComponent|SetAllBodiesBelowPhysicsBlendWeight (Variables|Default|GetSkeletalMesh) (Variables|Default|GetRagdollBone) _output_get false true)))

(fn ConstructionScript)

(fn GetHealth
  (return 0.0))

(fn GetPhysicsMesh
  (return (Variables|Default|GetSkeletalMesh)))

(fn TakeDamage
  (params (Damage :type Float%20%28double-precision%29))
  (bind _output_get (Variables|Default|SetHealth (- (Variables|Default|GetHealth) Damage)))
  (if (<= _output_get 0.0)
    (Variables|Default|SetRagdollBone "Hips")
    (Physics|SetSimulatePhysics (Variables|Default|GetSkeletalMesh) true)
    (else
      (Variables|Default|SetRagdollWeight 1.0)
      (bind _output_get_2 (Variables|Default|SetRagdollBone "Spine"))
      (Class|SkeletalMeshComponent|SetAllBodiesBelowSimulatePhysics (Variables|Default|GetSkeletalMesh) _output_get_2 true true)))
  (return (Variables|Default|GetSkeletalMesh) (Variables|Default|GetRagdollBone)))