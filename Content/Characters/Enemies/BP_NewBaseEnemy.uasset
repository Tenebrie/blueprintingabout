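; Base enemy character that handles target sensing and physics-driven hit and death reactions.
; UnitStatsComponent events drive the ragdoll: death simulates the body from the pelvis, while survived damage simulates from the spine, then eases back to animation on Tick.
; PawnSensing stores a living hostile unit as AggroPawn, or a non-hostile one as FollowPawn while no aggro target exists.
; OnTickUpdateAI runs every frame but is empty here.
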(event OnSeePawn(PawnSensing)
  (params (Pawn :type Pawn%20Object%20Reference))
  (bind (_isunit _unitstats) (CallFunction|GetActorUnitStats Pawn))
  (bind _unitalignment (Default|GetAlignment _unitstats))
  (if _isunit
    (if (Math|Boolean|ANDBoolean (not (Utilities|IsValid (Variables|Default|GetAggroPawn))) (CallFunction|IsEnemy _unitalignment (Default|GetAlignment (Variables|Default|GetUnitStatsComponent))) (> (.CurrentHealth (Default|GetHealth _unitstats)) 0.0))
      (Variables|Default|SetAggroPawn Pawn)
      (elif (and (not (Utilities|IsValid (Variables|Default|GetAggroPawn))) (not (CallFunction|IsEnemy _unitalignment (Default|GetAlignment (Variables|Default|GetUnitStatsComponent)))))
        (Variables|Default|SetFollowPawn Pawn)))))

(event OnDeath(UnitStatsComponent)
  (Variables|Default|SetRagdollWeight 1.0)
  (Variables|Default|SetRagdollBone "Pelvis")
  (Class|SkeletalMeshComponent|SetAllBodiesBelowSimulatePhysics (Variables|Character|GetMesh) (Variables|Default|GetRagdollBone) true true))

(event OnAfterDamageSurvived(UnitStatsComponent)
  (Variables|Default|SetRagdollWeight 0.5)
  (Variables|Default|SetRagdollBone "spine_01")
  (Class|SkeletalMeshComponent|SetAllBodiesBelowSimulatePhysics (Variables|Character|GetMesh) (Variables|Default|GetRagdollBone) true true))

(event Custom|OnTickUpdateRagdoll
  (if (and (> (Variables|Default|GetRagdollWeight) 0.0) (> (.CurrentHealth (Default|GetHealth (Variables|Default|GetUnitStatsComponent))) 0.0))
    (bind _output_get (Variables|Default|SetRagdollWeight (- (Variables|Default|GetRagdollWeight) (* (Variables|Default|GetDeltaSeconds) 1.0))))
    (if (> _output_get 0.0)
      (Class|SkeletalMeshComponent|SetAllBodiesBelowPhysicsBlendWeight (Variables|Character|GetMesh) (Variables|Default|GetRagdollBone) (Class|KismetMathLibrary|FInterpEaseinOut 0.0 1.0 _output_get 2.0) false true)
      (else
        (Class|SkeletalMeshComponent|SetAllBodiesBelowSimulatePhysics (Variables|Character|GetMesh) (Variables|Default|GetRagdollBone) false true)))))

(event Custom|OnTickUpdateAI)

(event EventBeginPlay
  (bind _mesh (Variables|Character|GetMesh))
  (Default|Init (Variables|Default|GetUnitStatsComponent) (Variables|Collision|GetCapsuleComponent) _mesh _mesh))

(event EventTick
  (params (DeltaSeconds :type Float%20%28single-precision%29))
  (Variables|Default|SetDeltaSeconds DeltaSeconds)
  (CallFunction|OnTickUpdateRagdoll)
  (CallFunction|OnTickUpdateAI))

(fn ConstructionScript)