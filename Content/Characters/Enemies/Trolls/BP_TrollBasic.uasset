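; Basic troll enemy that picks a random hand weapon, chases seen pawns and moves toward players it hears.
; Within melee range it opens a timed smack window in which weapon overlaps damage each player once.
; Damage triggers a physical hit reaction from the spine, eased back to animation on Tick.
; Death ragdolls from the pelvis, disables capsule collision and swaps the held weapon for a separate ragdoll mesh.
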(event OnSeePawn(PawnSensing)
  (params (Pawn :type Pawn%20Object%20Reference))
  (Variables|AILogic|SetAggroPawn Pawn))

(event OnHearNoise(PawnSensing)
  (params (Instigator :type Pawn%20Object%20Reference) (Location :type Vector%20%28by%20ref%29 :default "0, 0, 0") (Volume :type Float%20%28single-precision%29))
  (bind _asbp_player (Utilities|Casting|CastToBP_Player Instigator))
  (AI|AIMoveTo self "0, 0, 0" _asbp_player 5.0 false))

(event OnComponentBeginOverlap(WeaponMeshGameplay)
  (params (OverlappedComponent :type Primitive%20Component%20Object%20Reference) (OtherActor :type Actor%20Object%20Reference) (OtherComp :type Primitive%20Component%20Object%20Reference) (OtherBodyIndex :type Integer) (bFromSweep :type Boolean) (SweepResult :type Hit%20Result%20Structure%20%28by%20ref%29))
  (bind _asbp_player (Utilities|Casting|CastToBP_Player OtherActor))
  (if (and (Variables|AILogic|GetIsSmacking) (== (Utilities|Array|FindItem (Variables|AILogic|GetDamagedTargetsThisSmack) _asbp_player) -1))
    (Default|TakeDamage _asbp_player 3e+01)
    (Utilities|Array|AddUnique (Variables|AILogic|GetDamagedTargetsThisSmack) _asbp_player)))

(event Custom|OnDeath
  (Components|StaticMesh|SetStaticMesh (Variables|Default|GetWeaponMeshRagdoll) (Variables|/Script/Engine.StaticMeshComponent|GetStaticMesh (Variables|Default|GetWeaponMeshGameplay)))
  (Transformation|SetWorldTransform (Variables|Default|GetWeaponMeshRagdoll) (Transformation|GetWorldTransform (Variables|Default|GetWeaponMeshGameplay)) false true)
  (Components|DestroyComponent (Variables|Default|GetWeaponMeshGameplay)))

(event Custom|OnTickUpdateRagdoll
  (if (and (> (Variables|Default|GetRagdollWeight) 0.0) (> (Variables|Stats|GetHealth) 0.0))
    (bind _output_get (Variables|Default|SetRagdollWeight (- (Variables|Default|GetRagdollWeight) (* (Variables|Default|GetDeltaSeconds) 1.0))))
    (if (> _output_get 0.0)
      (Class|SkeletalMeshComponent|SetAllBodiesBelowPhysicsBlendWeight (Variables|Character|GetMesh) (Variables|Default|GetRagdollBone) (Class|KismetMathLibrary|FInterpEaseinOut 0.0 1.0 _output_get 2.0) false true)
      (else
        (Class|SkeletalMeshComponent|SetAllBodiesBelowSimulatePhysics (Variables|Character|GetMesh) (Variables|Default|GetRagdollBone) false true)))))

(event Custom|OnTickUpdateAI
  (if (and (Utilities|IsValid (Variables|AILogic|GetAggroPawn)) (not (Variables|AILogic|GetIsSmacking)))
    (if (< (Transformation|GetDistanceTo (Variables|AILogic|GetAggroPawn) self) 1.5e+02)
      (Variables|AILogic|SetIsSmacking true)
      (Utilities|FlowControl|Delay 2.4)
      (Variables|AILogic|SetIsSmacking false)
      (Utilities|Array|Clear (Variables|AILogic|GetDamagedTargetsThisSmack))
      (else
        (AI|AIMoveTo self "0, 0, 0" (Variables|AILogic|GetAggroPawn) 5.0 false)))))

(event EventBeginPlay
  (bind _asstatic_mesh (Utilities|Casting|CastToStaticMesh (.OutItem (Utilities|Array|Random (Utilities|Array|MakeArray "/Game/Characters/Enemies/Trolls/Weapons/SM_Wep_MutantGuy_01.SM_Wep_MutantGuy_01" "/Game/Characters/Enemies/Trolls/Weapons/SM_Wep_BigOrk_01.SM_Wep_BigOrk_01" "/Game/Characters/Enemies/Trolls/Weapons/SM_Wep_BarbarianGiant_01.SM_Wep_BarbarianGiant_01")))))
  (Components|StaticMesh|SetStaticMesh (Variables|Default|GetWeaponMeshGameplay) _asstatic_mesh)
  (Transformation|AttachComponentToComponent (Variables|Default|GetWeaponMeshGameplay) (Variables|Character|GetMesh) "RightHandSocket" "SnapToTarget" "SnapToTarget" "SnapToTarget" true))

(event EventTick
  (params (DeltaSeconds :type Float%20%28single-precision%29))
  (Variables|Default|SetDeltaSeconds DeltaSeconds)
  (CallFunction|OnTickUpdateRagdoll)
  (CallFunction|OnTickUpdateAI))

(fn ConstructionScript)

(fn GetAlignment
  (return "NewEnumerator2"))

(fn GetHealth
  (return (Variables|Stats|GetHealth)))

(fn GetMaxHealth
  (return (Variables|Stats|GetMaxHealth)))

(fn TakeDamage
  (params (Damage :type Float%20%28double-precision%29))
  (bind _output_get (Variables|Stats|SetHealth (- (Variables|Stats|GetHealth) Damage)))
  (if (<= _output_get 0.0)
    (Variables|Default|SetRagdollWeight 1.0)
    (Variables|Default|SetRagdollBone "Pelvis")
    (Collision|SetCollisionEnabled (Variables|Collision|GetCapsuleComponent) "NoCollision")
    (CallFunction|OnDeath)
    (else
      (Variables|Default|SetRagdollWeight 0.5)
      (bind _output_get_2 (Variables|Default|SetRagdollBone "spine_01"))))
  (Class|SkeletalMeshComponent|SetAllBodiesBelowSimulatePhysics (Variables|Character|GetMesh) _output_get_2 true true)
  (return (Variables|Character|GetMesh) (Variables|Default|GetRagdollBone) 1.0))