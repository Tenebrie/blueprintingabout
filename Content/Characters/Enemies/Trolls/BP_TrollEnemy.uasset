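; Troll melee enemy that spawns with a random oversized weapon in its right hand, dissolved on death.
; Each AI tick it chases its hostile aggro pawn, opens a timed smack window in close range, or otherwise falls back to a follow pawn.
; Weapon overlaps during a smack damage each living enemy once and switch aggro to it.
; Alignment changes clear both aggro and follow targets.
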(event OnComponentBeginOverlap(WeaponMeshGameplay)
  (params (OverlappedComponent :type Primitive%20Component%20Object%20Reference) (OtherActor :type Actor%20Object%20Reference) (OtherComp :type Primitive%20Component%20Object%20Reference) (OtherBodyIndex :type Integer) (bFromSweep :type Boolean) (SweepResult :type Hit%20Result%20Structure%20%28by%20ref%29))
  (bind (_isunit _unitstats) (CallFunction|GetActorUnitStats OtherActor))
  (if (CallFunction|IsAlive OtherActor)
    (if _isunit
      (if (CallFunction|IsEnemy (Default|GetAlignment _unitstats) (Default|GetAlignment (Variables|Default|GetEnemyStatsComponent)))
        (bind _aspawn (Utilities|Casting|CastToPawn OtherActor))
        (if (and (Variables|Default|GetIsSmacking) (== (Utilities|Array|FindItem (Variables|Default|GetDamagedTargetsThisSmack) _aspawn) -1))
          (Default|DealDamage (.UnitStats (CallFunction|GetActorUnitStats _aspawn)) (CallFunction|GetEnemyDI self 5.0 1e+01 "NewEnumerator1" "NewEnumerator0"))
          (Utilities|Array|AddUnique (Variables|Default|GetDamagedTargetsThisSmack) _aspawn)
          (Variables|Default|SetAggroPawn _aspawn))))))

(event OnDeath(EnemyStatsComponent)
  (CallFunction|DissolveMesh (Variables|Default|GetWeaponMeshGameplay))
  (Collision|SetCollisionEnabled (Variables|Default|GetWeaponMeshGameplay) "NoCollision"))

(event OnAlignmentChanged(EnemyStatsComponent)
  (params (NewAlignment :type E_UnitAlignment%20Enum :default "NewEnumerator0"))
  (Variables|Default|SetAggroPawn 0)
  (Variables|Default|SetFollowPawn 0))

(event EventBeginPlay
  (|CallParentFunction)
  (bind _asstatic_mesh (Utilities|Casting|CastToStaticMesh (.OutItem (Utilities|Array|Random (Utilities|Array|MakeArray "/Game/Characters/Enemies/Trolls/Weapons/SM_Wep_MutantGuy_01.SM_Wep_MutantGuy_01" "/Game/Characters/Enemies/Trolls/Weapons/SM_Wep_BigOrk_01.SM_Wep_BigOrk_01" "/Game/Characters/Enemies/Trolls/Weapons/SM_Wep_BarbarianGiant_01.SM_Wep_BarbarianGiant_01")))))
  (Components|StaticMesh|SetStaticMesh (Variables|Default|GetWeaponMeshGameplay) _asstatic_mesh)
  (Transformation|AttachComponentToComponent (Variables|Default|GetWeaponMeshGameplay) (Variables|Character|GetMesh) "RightHandSocket" "SnapToTarget" "SnapToTarget" "SnapToTarget" true))

(event EventOnTickUpdateAI
  (|CallParentFunction)
  (if (and (Utilities|IsValid (Variables|Default|GetAggroPawn)) (CallFunction|IsAlive self))
    (if (CallFunction|IsEnemy (Default|GetAlignment (.UnitStats (CallFunction|GetActorUnitStats (Variables|Default|GetAggroPawn)))) (Default|GetAlignment (Variables|Default|GetEnemyStatsComponent)))
      (if (> (.CurrentHealth (Default|GetHealth (.UnitStats (CallFunction|GetActorUnitStats (Variables|Default|GetAggroPawn))))) 0.0)
        (if (not (Variables|Default|GetIsSmacking))
          (if (< (Transformation|GetDistanceTo (Variables|Default|GetAggroPawn) self) 1.5e+02)
            (Variables|Default|SetIsSmacking true)
            (Utilities|FlowControl|Delay 2.4)
            (Variables|Default|SetIsSmacking false)
            (Utilities|Array|Clear (Variables|Default|GetDamagedTargetsThisSmack))
            (else
              (AI|AIMoveTo self "0, 0, 0" (Variables|Default|GetAggroPawn) 5e+01 false))))
        (else
          (Variables|Default|SetAggroPawn 0)
          (if (Utilities|IsValid (Variables|Default|GetFollowPawn)) :!label _label
            (AI|AIMoveTo self "0, 0, 0" (Variables|Default|GetFollowPawn) 5e+01 false))))
      (else
        (Variables|Default|SetAggroPawn 0)))
    (else
      (goto _label))))

(fn ConstructionScript
  (|CallParentFunction))