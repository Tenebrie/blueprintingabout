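; Base enemy Blueprint that handles damage with physical hit reactions and ragdoll death.
; TakeDamage reduces Health, simulates physics below the spine on a hit or below the hips on death, disables capsule collision when lethal, and returns mesh, bone and multiplier for applying force.
; While the enemy lives, Tick eases the physics blend weight back to animation, then stops simulation.
; GetHealth returns a constant zero rather than Health.
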(event EventTick
  (params (DeltaSeconds :type Float%20%28single-precision%29))
  (if (and (> (Variables|Default|GetRagdollWeight) 0.0) (> (Variables|Default|GetHealth) 0.0))
    (bind _output_get (Variables|Default|SetRagdollWeight (- (Variables|Default|GetRagdollWeight) (* DeltaSeconds 1.0))))
    (if (> _output_get 0.0)
      (Class|SkeletalMeshComponent|SetAllBodiesBelowPhysicsBlendWeight (Variables|Default|GetSkeletalMesh) (Variables|Default|GetRagdollBone) (Class|KismetMathLibrary|FInterpEaseinOut 0.0 1.0 _output_get 2.0) false true)
      (else
        (Class|SkeletalMeshComponent|SetAllBodiesBelowSimulatePhysics (Variables|Default|GetSkeletalMesh) (Variables|Default|GetRagdollBone) false true)))))

(fn ConstructionScript)

(fn GetHealth
  (return 0.0))

(fn GetPhysicsMesh
  (return (Variables|Default|GetSkeletalMesh)))

(fn TakeDamage
  (params (Damage :type Float%20%28double-precision%29))
  (bind _output_get (Variables|Default|SetHealth (- (Variables|Default|GetHealth) Damage)))
  (if (<= _output_get 0.0)
    (Variables|Default|SetRagdollWeight 1.0)
    (Variables|Default|SetRagdollBone "Hips")
    (Collision|SetCollisionEnabled (Variables|Default|GetCapsuleCollider) "NoCollision")
    (else
      (Variables|Default|SetRagdollWeight 0.5)
      (bind _output_get_2 (Variables|Default|SetRagdollBone "Spine"))))
  (Class|SkeletalMeshComponent|SetAllBodiesBelowSimulatePhysics (Variables|Default|GetSkeletalMesh) _output_get_2 true true)
  (return (Variables|Default|GetSkeletalMesh) (Variables|Default|GetRagdollBone) 1.0))