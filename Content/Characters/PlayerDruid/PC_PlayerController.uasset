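; Player controller for the druid character, managing the main UI, spell loadout and respawning.
; BeginPlay builds a hardcoded spell map, creates a slot component per binding, registers both with the UI and assigns two default spells.
; While the pawn lives, held primary, secondary and movement inputs open gates that tick their slots.
; It also relays global cooldowns and UI info, and respawns a dead pawn at a PlayerStart, re-linking slots and UI.
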(event Custom|OnTickPrimaryAction
  (bind _spellslots (Variables|Default|GetSpellSlots))
  (bind _value (Utilities|Map|Find _spellslots "NewEnumerator0"))
  (Utilities|FlowControl|Gate true
    (:Exit
      (if (Utilities|IsValid _value)
        (Default|OnTickPrimaryAction _value)))))

(event Custom|OnTickSecondaryAction
  (bind _spellslots (Variables|Default|GetSpellSlots))
  (bind _value (Utilities|Map|Find _spellslots "NewEnumerator1"))
  (Utilities|FlowControl|Gate true
    (:Exit
      (if (Utilities|IsValid _value)
        (Default|OnTickSecondaryAction _value)))))

(event Custom|OnTickMovementAction
  (bind _spellslots (Variables|Default|GetSpellSlots))
  (bind _value (Utilities|Map|Find _spellslots "NewEnumerator3"))
  (Utilities|FlowControl|Gate true
    (:Exit
      (if (Utilities|IsValid _value)
        (Default|OnTickMovementAction _value)))))

(event EventBeginPlay
  (bind _returnvalue (UserInterface|CreateWidget "/Game/Systems/UserInterface/UI_Main.UI_Main_C" self))
  (bind _output_get (Variables|Default|SetPlayerUIRef _returnvalue))
  (UserInterface|Viewport|AddtoViewport _output_get 0)
  (Init|InitSpells)
  (bind _enumvalue (|ForEachE_SpellSlotBinding)
    (:LoopBody
      (bind _returnvalue_2 (AddComponent|AddBPCSpellSlot _enumvalue self "NewEnumerator0"))
      (Utilities|Map|Add (Variables|Default|GetSpellSlots) _enumvalue _returnvalue_2)
      (Default|RegisterSpellSlot (Variables|/Game/Systems/InventorySystem/UI_InventoryMain.UI_InventoryMain_C|GetSpellsTab (Variables|/Game/Systems/UserInterface/UI_Main.UI_Main_C|GetInventoryComponent (Variables|Default|GetPlayerUIRef))) _returnvalue_2)
      (Default|RegisterSpellSlot (Variables|/Game/Systems/UserInterface/UI_Main.UI_Main_C|GetSpellsHotbarComponent (Variables|Default|GetPlayerUIRef)) _returnvalue_2))
    (:then
      (Default|AssignSpell (.Value (Utilities|Map|Find (Variables|Default|GetSpellSlots) "NewEnumerator0")) (.Value (Utilities|Map|Find (Variables|Default|GetSpells) "NewEnumerator0")))
      (Default|AssignSpell (.Value (Utilities|Map|Find (Variables|Default|GetSpellSlots) "NewEnumerator1")) (.Value (Utilities|Map|Find (Variables|Default|GetSpells) "NewEnumerator4")))
      (bind _values (Utilities|Map|Values (Variables|Default|GetSpells)))
      (for _array_element _values
        (Default|RegisterSpell (Variables|/Game/Systems/InventorySystem/UI_InventoryMain.UI_InventoryMain_C|GetSpellsTab (Variables|/Game/Systems/UserInterface/UI_Main.UI_Main_C|GetInventoryComponent (Variables|Default|GetPlayerUIRef))) _array_element)))))

(event EventTick
  (params (DeltaSeconds :type Float%20%28single-precision%29))
  (Variables|Default|SetDeltaSeconds DeltaSeconds)
  (if (CallFunction|IsAlive (Pawn|GetControlledPawn))
    (CallFunction|OnTickMovementAction)
    (CallFunction|OnTickPrimaryAction)
    (CallFunction|OnTickSecondaryAction)))

(event Input|ActionEvents|InputActionPrimaryAction
  (params (Key :type Key%20Structure :default "None"))
  (bind _spellslots (Variables|Default|GetSpellSlots))
  (bind _value (Utilities|Map|Find _spellslots "NewEnumerator0"))
  (:Pressed
    (Utilities|FlowControl|Gate true) ; enters at Open
  )
  (:Released
    (Utilities|FlowControl|Gate true) ; enters at Close
  ))

(event Input|ActionEvents|InputActionRespawnKey
  (params (Key :type Key%20Structure :default "None"))
  (:Pressed
    (if (CallFunction|IsDead (Pawn|GetControlledPawn))
      (CallFunction|RespawnPawn))))

(event Input|ActionEvents|InputActionSecondaryAction
  (params (Key :type Key%20Structure :default "None"))
  (bind _spellslots (Variables|Default|GetSpellSlots))
  (bind _value (Utilities|Map|Find _spellslots "NewEnumerator1"))
  (:Pressed
    (Utilities|FlowControl|Gate true) ; enters at Open
  )
  (:Released
    (Utilities|FlowControl|Gate true) ; enters at Close
  ))

(event Input|ActionEvents|InputActionMovementAction
  (params (Key :type Key%20Structure :default "None"))
  (bind _spellslots (Variables|Default|GetSpellSlots))
  (bind _value (Utilities|Map|Find _spellslots "NewEnumerator3"))
  (:Pressed
    (Utilities|FlowControl|Gate true) ; enters at Open
  )
  (:Released
    (Utilities|FlowControl|Gate true) ; enters at Close
  ))

(fn ConstructionScript)

(fn InitSpells
  (Utilities|Map|Add (Variables|Default|GetSpells) "NewEnumerator0" (Utilities|Struct|MakeS_Spell "Fireball" "This spell is good to toss at things you want to be burnity." (Utilities|Set|MakeSet "NewEnumerator0" "NewEnumerator1") "/Game/Abilities/Fireball/Icon_Fireball.Icon_Fireball" "/Game/Abilities/Fireball/BPC_FireballController.BPC_FireballController_C"))
  (Utilities|Map|Add (Variables|Default|GetSpells) "NewEnumerator1" (Utilities|Struct|MakeS_Spell "Rockball" "This spell is good to toss at things you want to sent flying." (Utilities|Set|MakeSet "NewEnumerator0" "NewEnumerator1") "/Game/Abilities/Rockball/Icon_RockThrow.Icon_RockThrow" "/Game/Abilities/Rockball/BPC_RockThrowController.BPC_RockThrowController_C"))
  (Utilities|Map|Add (Variables|Default|GetSpells) "NewEnumerator2" (Utilities|Struct|MakeS_Spell "Fan of Knives" "Whoosh" (Utilities|Set|MakeSet "NewEnumerator0" "NewEnumerator1") "/Game/Abilities/FanOfKnives/Icon_FanOfKnives.Icon_FanOfKnives" "/Game/Abilities/FanOfKnives/BPC_FanOfKnives_Controller.BPC_FanOfKnives_Controller_C"))
  (Utilities|Map|Add (Variables|Default|GetSpells) "NewEnumerator3" (Utilities|Struct|MakeS_Spell "Charm" "From Bezllikii with love <3" (Utilities|Set|MakeSet "NewEnumerator0") "/Game/Abilities/Charm/Icon_Charm.Icon_Charm" "/Game/Abilities/Charm/BPC_CharmController.BPC_CharmController_C"))
  (Utilities|Map|Add (Variables|Default|GetSpells) "NewEnumerator4" (Utilities|Struct|MakeS_Spell "Magic Fountain" "Pewpewpew" (Utilities|Set|MakeSet "NewEnumerator0") "/Game/Abilities/Charm/Icon_Charm.Icon_Charm" "/Game/Abilities/MagicFountain/BPC_MagicFountainController.BPC_MagicFountainController_C")))

(fn StartGlobalCooldown
  (params (Time :type Float%20%28double-precision%29))
  (bind _values (Utilities|Map|Values (Variables|Default|GetSpellSlots)))
  (for _array_element _values
    (Default|StartGlobalCooldown _array_element Time)))

(fn ShowHoverInfo
  (params (Agent :type Hover%20Info%20Agent%20Object%20Reference))
  (Default|UpdatefromAgent (Variables|/Game/Systems/UserInterface/UI_Main.UI_Main_C|GetHoverInfoComponent (Variables|Default|GetPlayerUIRef)) Agent))

(fn HideHoverInfo
  (Default|UpdatefromAgent (Variables|/Game/Systems/UserInterface/UI_Main.UI_Main_C|GetHoverInfoComponent (Variables|Default|GetPlayerUIRef))))

(fn ShowInventorySpellDescription
  (params (SpellData :type S%20Spell%20Structure))
  (Default|SetData (Variables|/Game/Systems/InventorySystem/Abilities/UI_SpellsTab.UI_SpellsTab_C|GetUI_SpellDescription (Variables|/Game/Systems/InventorySystem/UI_InventoryMain.UI_InventoryMain_C|GetSpellsTab (Variables|/Game/Systems/UserInterface/UI_Main.UI_Main_C|GetInventoryComponent (Variables|Default|GetPlayerUIRef)))) SpellData))

(fn RespawnPawn
  (LocalVariables|SetPreviousPawn (Pawn|GetControlledPawn))
  (bind _returnvalue (Actor|GetActorOfClass "/Script/Engine.PlayerStart"))
  (bind _returnvalue_2 (Game|SpawnActorfromClass "/Game/Characters/PlayerDruid/BP_Player.BP_Player_C" (Math|Conversions|ToTransform(Vector) (Transformation|GetActorLocation _returnvalue)) "Undefined" 0 0))
  (LocalVariables|SetCreatedPawn _returnvalue_2)
  (Pawn|Possess (LocalVariables|GetCreatedPawn))
  (Variables|/Game/Systems/UserInterface/UI_Main.UI_Main_C|SetPlayerRef (Variables|Default|GetPlayerUIRef) (LocalVariables|GetCreatedPawn))
  (bind _values (Utilities|Map|Values (Variables|Default|GetSpellSlots)))
  (for _array_element _values
    (Default|UpdatePawn _array_element (LocalVariables|GetCreatedPawn)))
  (Actor|DestroyActor (LocalVariables|GetPreviousPawn)))