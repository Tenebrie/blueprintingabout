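; Charm ability controller that changes the alignment of the enemy nearest the player's cursor.
; At the active spell's cast point it starts the global cooldown, whether or not a target is found.
; It traces under the cursor and searches unit-tagged actors for the closest enemy within a short radius of the hit.
; A found enemy gets its stats' alignment set and a charm effect attached to its root.
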(event EventBeginPlay
  (|CallParentFunction) ; This node is disabled and will not be called.\nDrag off pins to build functionality.
)

(event EventTick
  (params (DeltaSeconds :type Float%20%28single-precision%29)))

(event EventOnActiveSpellCastPoint
  (Default|StartGlobalCooldown (Variables|Default|GetPlayerController) 0.5)
  (bind _outactors (Actor|GetAllActorswithTag (CallFunction|GetTagbyValue "(TagName=\"is_unit\")")))
  (bind (_hasvalue _closestenemy _closestenemystats) (CallFunction|GetClosestEnemytoPoint (.Location (Collision|BreakHitResult (.HitResult (Game|Player|GetHitResultUnderCursorbyChannel (Variables|Default|GetPlayerController) "TraceTypeQuery1" true)))) _outactors "NewEnumerator0" 2e+02))
  (if _hasvalue
    (Default|SetAlignment _closestenemystats "NewEnumerator0")
    (Niagara|SpawnSystemAttached "/Game/Abilities/Charm/FX_CharmTargetCast.FX_CharmTargetCast" (Variables|/Script/Engine.Actor|GetRootComponent _closestenemy) "None" "0, 0, 0" "0, 0, 0" "KeepRelativeOffset" true)))