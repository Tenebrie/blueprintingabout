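; Base ability controller component for BP_Player, providing projectile casting, cooldown tracking and placeholder active, passive and movement spell events.
; Launch requests check CanCast, then choose the hand from cursor angle versus velocity, or alternate when stationary.
; Cast-speed-scaled delays and animation rate time spawning at the hand socket, detaching and releasing toward the cursor.
; Cooldown starts after recovery; LaunchProjectileAtPoint ignores its Target, as aim re-reads the cursor at release.
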(event Custom|OnSpellCastAsMovement
  (Development|PrintString "Please Implement Me"))

(event Custom|OnProjectileLaunched
  (params (Launch%20Args :type S%20Projectile%20Launch%20Args%20Structure))
  (bind (_projectile _castspeed _cooldown) (Utilities|Struct|BreakS_ProjectileLaunchArgs Launch%20Args))
  (Variables|SingleUse|SetProjectileLaunchClass _projectile)
  (Variables|SingleUse|SetProjectileLaunchCooldown _cooldown)
  (Variables|SingleUse|SetProjectileLaunchCastSpeed _castspeed)
  (Variables|/Game/Characters/PlayerCharacter/BP_Player.BP_Player_C|SetCurrentCastIndex (Variables|Default|GetPlayerBlueprint) (+ (Variables|/Game/Characters/PlayerCharacter/BP_Player.BP_Player_C|GetCurrentCastIndex (Variables|Default|GetPlayerBlueprint)) 1))
  (Utilities|FlowControl|Sequence
    (:then_0
      (bind _aspc_player_controller (Utilities|Casting|CastToPC_PlayerController (Pawn|GetController (Variables|Default|GetPlayerBlueprint))))
      (if (> (Math|Vector|VectorLength (Transformation|GetVelocity (Variables|Default|GetPlayerBlueprint))) 0.0)
        (Variables|/Game/Characters/PlayerCharacter/BP_Player.BP_Player_C|SetIsCastingLeftHand (Variables|Default|GetPlayerBlueprint) (< (CallFunction|GetAngleBetweenVectors (Math|Vector|MakeVector (.X (Class|KismetMathLibrary|BreakVector3f (Math|Vector|GetUnitDirection(Vector) (Transformation|GetActorLocation (Variables|Default|GetPlayerBlueprint)) (.Location (Collision|BreakHitResult (.HitResult (Game|Player|GetHitResultUnderCursorbyChannel _aspc_player_controller "TraceTypeQuery1" true))))))) (.Y (Class|KismetMathLibrary|BreakVector3f (Math|Vector|GetUnitDirection(Vector) (Transformation|GetActorLocation (Variables|Default|GetPlayerBlueprint)) (.Location (Collision|BreakHitResult (.HitResult (Game|Player|GetHitResultUnderCursorbyChannel _aspc_player_controller "TraceTypeQuery1" true))))))) 0.0) (Transformation|GetVelocity (Variables|Default|GetPlayerBlueprint))) 0.0))
        (else
          (Variables|/Game/Characters/PlayerCharacter/BP_Player.BP_Player_C|SetIsCastingLeftHand (Variables|Default|GetPlayerBlueprint) (not (Variables|/Game/Characters/PlayerCharacter/BP_Player.BP_Player_C|GetIsCastingLeftHand (Variables|Default|GetPlayerBlueprint)))))))
    (:then_1
      (Variables|/Script/Engine.SkeletalMeshComponent|SetGlobalAnimRateScale (Variables|/Script/Engine.Character|GetMesh (Variables|Default|GetPlayerBlueprint)) (Variables|SingleUse|GetProjectileLaunchCastSpeed))
      (bind _asplayer_controller (Utilities|Casting|CastToPlayerController (Pawn|GetController (Variables|Default|GetPlayerBlueprint))))
      (Utilities|FlowControl|Delay (/ 0.18 (Variables|SingleUse|GetProjectileLaunchCastSpeed)))
      (bind _returnvalue (Game|SpawnActorfromClass (Variables|SingleUse|GetProjectileLaunchClass) (Transformation|GetActorTransform (Variables|Default|GetPlayerBlueprint)) "Undefined" 0 self 0))
      (bind _output_get (Variables|SingleUse|SetLastSpawnedProjectile _returnvalue))
      (Transformation|AttachComponentToComponent _output_get (Variables|/Script/Engine.Character|GetMesh (Variables|Default|GetPlayerBlueprint)) (Utilities|String|StringToName (Utilities|String|SelectString "LeftHandSocket" "MainHandSocket" (Variables|/Game/Characters/PlayerCharacter/BP_Player.BP_Player_C|GetIsCastingLeftHand (Variables|Default|GetPlayerBlueprint)))) "SnapToTarget" "SnapToTarget" "SnapToTarget" true)
      (Utilities|FlowControl|Delay (/ 0.2 (Variables|SingleUse|GetProjectileLaunchCastSpeed)))
      (Transformation|DetachFromActor (Variables|SingleUse|GetLastSpawnedProjectile) "KeepWorld" "KeepWorld" "KeepWorld")
      (Transformation|SetActorRotation (Variables|SingleUse|GetLastSpawnedProjectile) (Math|Conversions|RotationFromXVector (Math|Vector|GetUnitDirection(Vector) (Transformation|GetActorLocation (Variables|SingleUse|GetLastSpawnedProjectile)) (Math|Vector|MakeVector (.X (Class|KismetMathLibrary|BreakVector3f (.Location (Collision|BreakHitResult (.HitResult (Game|Player|GetHitResultUnderCursorbyChannel _asplayer_controller "TraceTypeQuery1" true)))))) (.Y (Class|KismetMathLibrary|BreakVector3f (.Location (Collision|BreakHitResult (.HitResult (Game|Player|GetHitResultUnderCursorbyChannel _asplayer_controller "TraceTypeQuery1" true)))))) (.Z (Class|KismetMathLibrary|BreakVector3f (Transformation|GetActorLocation (Variables|SingleUse|GetLastSpawnedProjectile))))))))
      (Default|SetProjectileStateandNotify (Variables|SingleUse|GetLastSpawnedProjectile) "NewEnumerator1")
      (Utilities|FlowControl|Delay (/ 0.3 (Variables|SingleUse|GetProjectileLaunchCastSpeed)))
      (Variables|/Game/Characters/PlayerCharacter/BP_Player.BP_Player_C|SetIsCasting (Variables|Default|GetPlayerBlueprint) false)
      (Utilities|FlowControl|Delay (/ 0.0 (Variables|SingleUse|GetProjectileLaunchCastSpeed)))
      (Variables|/Script/Engine.SkeletalMeshComponent|SetGlobalAnimRateScale (Variables|/Script/Engine.Character|GetMesh (Variables|Default|GetPlayerBlueprint)) 1.0)
      (Variables|/Game/Characters/PlayerCharacter/BP_Player.BP_Player_C|SetCanCast (Variables|Default|GetPlayerBlueprint) true)
      (Variables|Default|SetRemainingCooldown (Math|Float|Max(Float) (Variables|SingleUse|GetProjectileLaunchCooldown) 0.0)))))

(event Custom|OnEventTick
  (params (DeltaSeconds :type Float%20%28double-precision%29))
  (Variables|Default|SetRemainingCooldown (Math|Float|Max(Float) (- (Variables|Default|GetRemainingCooldown) DeltaSeconds) 0.0)))

(event Custom|OnSpellCastAsActive
  (Development|PrintString "Please Implement Me"))

(event Custom|OnSpellCastAsPassive
  (Development|PrintString "Please Implement Me"))

(event EventBeginPlay
  (bind _asbp_player (Utilities|Casting|CastToBP_Player (Components|GetOwner)))
  (Variables|Default|SetPlayerBlueprint _asbp_player))

(fn LaunchProjectileatPoint
  (params (Target :type Vector%203f%20Structure) (LaunchArgs :type S%20Projectile%20Launch%20Args%20Structure))
  (if (Variables|/Game/Characters/PlayerCharacter/BP_Player.BP_Player_C|GetCanCast (Variables|Default|GetPlayerBlueprint))
    (Variables|/Game/Characters/PlayerCharacter/BP_Player.BP_Player_C|SetIsCasting (Variables|Default|GetPlayerBlueprint) true)
    (Variables|/Game/Characters/PlayerCharacter/BP_Player.BP_Player_C|SetCanCast (Variables|Default|GetPlayerBlueprint) false)
    (CallFunction|OnProjectileLaunched LaunchArgs)))

(fn LaunchProjectileatMouse
  (params (LaunchArgs :type S%20Projectile%20Launch%20Args%20Structure))
  (bind _asplayer_controller (Utilities|Casting|CastToPlayerController (Pawn|GetController (Variables|Default|GetPlayerBlueprint))))
  (CallFunction|LaunchProjectileatPoint (.Location (Collision|BreakHitResult (.HitResult (Game|Player|GetHitResultUnderCursorbyChannel _asplayer_controller "TraceTypeQuery1" true)))) LaunchArgs))

(fn IsReadytoCast
  (return (<= (Variables|Default|GetRemainingCooldown) 0.0)))

(fn GetAngleBetweenVectors
  (params (A :type Vector) (B :type Vector%203f%20Structure))
  (bind (_x _y) (Math|Vector|BreakVector A))
  (bind (_x_2 _y_2) (Class|KismetMathLibrary|BreakVector3f B))
  (return (Class|KismetMathLibrary|DegAtan2 (- (* _x _y_2) (* _y _x_2)) (+ (* _x _x_2) (* _y _y_2)))))