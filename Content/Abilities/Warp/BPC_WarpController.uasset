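; Warp spell component that teleports its owning pawn to the point under the mouse cursor.
; On the cast point event, it adds the owner's height above ground, found by a downward trace, to the cursor hit location.
; It spawns a Niagara effect facing the destination at the origin and attaches another after teleporting.
; Each rune of one type halves the cooldown and doubles the mana cost.
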(event EventBeginPlay
  (|CallParentFunction) ; This node is disabled and will not be called.\nDrag off pins to build functionality.
)

(event EventTick
  (params (DeltaSeconds :type Float%20%28single-precision%29)))

(event EventOnActiveSpellCastPoint
  (bind _returnvalue (Components|GetOwner))
  (bind _returnvalue_2 (Components|GetOwner))
  (bind _returnvalue_3 (Components|GetOwner))
  (bind _returnvalue_4 (Transformation|GetActorLocation _returnvalue_2))
  (bind _returnvalue_5 (Transformation|GetActorLocation _returnvalue_3))
  (bind _aspawn (Utilities|Casting|CastToPawn _returnvalue))
  (bind _returnvalue_6 (Pawn|GetController _aspawn))
  (bind _asplayer_controller (Utilities|Casting|CastToPlayerController _returnvalue_6))
  (bind (_hitresult _returnvalue_7) (Game|Player|GetHitResultUnderCursorbyChannel _asplayer_controller "TraceTypeQuery1" true))
  (bind _location (Collision|BreakHitResult _hitresult))
  (bind (_x _y _z) (Math|Vector|BreakVector _location))
  (bind (_outhit _returnvalue_8) (Collision|LineTraceByChannel _returnvalue_5 (+ _returnvalue_5 "0,0,-5000.000000") "TraceTypeQuery1" false (Utilities|Array|MakeArray (Components|GetOwner)) "None"))
  (if _returnvalue_7
    (Niagara|SpawnSystematLocation "/Game/Abilities/Warp/FX_WarpSpellSource.FX_WarpSpellSource" _returnvalue_4 (Math|Rotator|MakeRotfromX (Math|Vector|GetUnitDirection(Vector) _returnvalue_4 (Math|Vector|MakeVector _x _y (+ _z (- (.Z (Math|Vector|BreakVector (Transformation|GetActorLocation _returnvalue))) (.Z (Math|Vector|BreakVector (.Location (Collision|BreakHitResult _outhit))))) 0.0)))))
    (Transformation|SetActorLocation _returnvalue_3 (Math|Vector|MakeVector _x _y (+ _z (- (.Z (Math|Vector|BreakVector (Transformation|GetActorLocation _returnvalue))) (.Z (Math|Vector|BreakVector (.Location (Collision|BreakHitResult _outhit))))) 0.0)) false true)
    (Niagara|SpawnSystemAttached "/Game/Abilities/Warp/FX_WarpSpellTarget.FX_WarpSpellTarget" (Variables|/Script/Engine.Actor|GetRootComponent (Components|GetOwner)) "None" "0, 0, 0" "0, 0, 0" "KeepRelativeOffset" true)))

(fn GetDescriptionFields
  (return (Utilities|Struct|MakeS_SpellDescriptionFields "Warp" "For the cases when you wanna go... just go.")))

(fn GetActiveSpellCooldown
  (return (/ (Math|Float|MakeLiteralFloat 1.0) (Math|Float|Power 2.0 (Math|Conversions|ToFloat(Integer) (.RuneCount (CallFunction|GetRuneStatus "NewEnumerator3")))))))

(fn GetManaCost
  (return (* (Math|Float|MakeLiteralFloat 12.0) (Math|Float|Power 2.0 (Math|Conversions|ToFloat(Integer) (.RuneCount (CallFunction|GetRuneStatus "NewEnumerator3")))))))