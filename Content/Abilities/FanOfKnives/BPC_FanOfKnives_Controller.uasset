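; Ability controller component for Fan of Knives, which throws a symmetric spread of knife projectiles from the player toward the cursor.
; On the active spell cast point, it traces under the cursor and flattens that hit to the player's height.
; It launches one center knife at that point, then a loop adds mirrored pairs by rotating the aim direction around vertical in even steps up to the maximum half angle.
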(event EventBeginPlay
  (|CallParentFunction) ; This node is disabled and will not be called.\nDrag off pins to build functionality.
)

(event EventTick
  (params (DeltaSeconds :type Float%20%28single-precision%29)))

(event EventOnActiveSpellCastPoint
  (bind _asbp_player (Utilities|Casting|CastToBP_Player (Components|GetOwner)))
  (Variables|Default|SetPawn _asbp_player)
  (bind _aspc_player_controller (Utilities|Casting|CastToPC_PlayerController (Pawn|GetController _asbp_player)))
  (CallFunction|LaunchProjectileatPoint "/Game/Abilities/FanOfKnives/BP_FanOfKnives_Projectile.BP_FanOfKnives_Projectile_C" (Transformation|GetActorLocation (Variables|Default|GetPawn)) (Math|Vector|MakeVector (.X (Math|Vector|BreakVector (.Location (Collision|BreakHitResult (.HitResult (Game|Player|GetHitResultUnderCursorbyChannel _aspc_player_controller "TraceTypeQuery1" true)))))) (.Y (Math|Vector|BreakVector (.Location (Collision|BreakHitResult (.HitResult (Game|Player|GetHitResultUnderCursorbyChannel _aspc_player_controller "TraceTypeQuery1" true)))))) (.Z (Math|Vector|BreakVector (Transformation|GetActorLocation (Variables|Default|GetPawn))))) "NewEnumerator0" "NewEnumerator1")
  (for _index (range 1 (Variables|Default|GetProjectileHalfCount))
    (CallFunction|LaunchProjectileatPoint "/Game/Abilities/FanOfKnives/BP_FanOfKnives_Projectile.BP_FanOfKnives_Projectile_C" (Transformation|GetActorLocation (Variables|Default|GetPawn)) (+ (Math|Vector|RotateVectorAroundAxis (Math|Vector|GetUnitDirection(Vector) (Transformation|GetActorLocation (Variables|Default|GetPawn)) (Math|Vector|MakeVector (.X (Math|Vector|BreakVector (.Location (Collision|BreakHitResult (.HitResult (Game|Player|GetHitResultUnderCursorbyChannel _aspc_player_controller "TraceTypeQuery1" true)))))) (.Y (Math|Vector|BreakVector (.Location (Collision|BreakHitResult (.HitResult (Game|Player|GetHitResultUnderCursorbyChannel _aspc_player_controller "TraceTypeQuery1" true)))))) (.Z (Math|Vector|BreakVector (Transformation|GetActorLocation (Variables|Default|GetPawn)))))) (* (/ (Variables|Default|GetMaxSpreadHalfAngle) (Variables|Default|GetProjectileHalfCount)) _index) "0, 0,-1.000000") (Transformation|GetActorLocation (Variables|Default|GetPawn))) "NewEnumerator0" "NewEnumerator1")
    (CallFunction|LaunchProjectileatPoint "/Game/Abilities/FanOfKnives/BP_FanOfKnives_Projectile.BP_FanOfKnives_Projectile_C" (Transformation|GetActorLocation (Variables|Default|GetPawn)) (+ (Math|Vector|RotateVectorAroundAxis (Math|Vector|GetUnitDirection(Vector) (Transformation|GetActorLocation (Variables|Default|GetPawn)) (Math|Vector|MakeVector (.X (Math|Vector|BreakVector (.Location (Collision|BreakHitResult (.HitResult (Game|Player|GetHitResultUnderCursorbyChannel _aspc_player_controller "TraceTypeQuery1" true)))))) (.Y (Math|Vector|BreakVector (.Location (Collision|BreakHitResult (.HitResult (Game|Player|GetHitResultUnderCursorbyChannel _aspc_player_controller "TraceTypeQuery1" true)))))) (.Z (Math|Vector|BreakVector (Transformation|GetActorLocation (Variables|Default|GetPawn)))))) (* (/ (Variables|Default|GetMaxSpreadHalfAngle) (Variables|Default|GetProjectileHalfCount)) _index) "0, 0,1.000000") (Transformation|GetActorLocation (Variables|Default|GetPawn))) "NewEnumerator0" "NewEnumerator1")))