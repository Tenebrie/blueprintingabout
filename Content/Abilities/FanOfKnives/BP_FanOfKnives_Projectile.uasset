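; Knife projectile for the Fan of Knives ability that deals damage scaling with Impale stacks on the target.
; Hitting a target adds one BPC_ImpaleBuff stack and dissolves the knife mesh; hitting an obstacle only dissolves it, more slowly.
; The GetDamage function returns rounded base damage plus the target's Impale buff intensity times the rounded per-stack damage, with full weapon scaling.
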(event EventOnTargetHit
  (params (Target :type Actor%20Object%20Reference))
  (CallFunction|CreateBuff "/Game/Abilities/FanOfKnives/BPC_ImpaleBuff.BPC_ImpaleBuff_C" Target 1)
  (CallFunction|DissolveMesh (Variables|Default|GetKnife) 2.0 false))

(event EventOnObstacleHit
  (CallFunction|DissolveMesh (Variables|Default|GetKnife) 1.0 false))

(fn ConstructionScript
  (|CallParentFunction))

(fn GetDamage
  (params (DamageImpactTarget :type Actor%20Object%20Reference))
  (return (Math|Conversions|ToFloat(Integer) (+ (* (CallFunction|GetBuffIntensity "/Game/Abilities/FanOfKnives/BPC_ImpaleBuff.BPC_ImpaleBuff_C" DamageImpactTarget) (Math|Float|Round (Variables|Default|GetImpale_DamagePerStack))) (Math|Float|Round (Variables|Default|GetBaseDamage)))) 1.0 "NewEnumerator1"))