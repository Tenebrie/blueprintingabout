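; Short-lived hitbox actor for the Spirit Slash ability that detects enemies caught in the slash.
; It destroys itself one tick after BeginPlay, so only overlaps during that brief window register.
; Static mesh overlaps are filtered to units of hostile alignment and reported to the SpellController through OnEnemyHit.
; A DamagedActors list prevents the same enemy from being reported twice.
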(event OnComponentBeginOverlap(StaticMesh)
  (params (OverlappedComponent :type Primitive%20Component%20Object%20Reference) (OtherActor :type Actor%20Object%20Reference) (OtherComp :type Primitive%20Component%20Object%20Reference) (OtherBodyIndex :type Integer) (bFromSweep :type Boolean) (SweepResult :type Hit%20Result%20Structure%20%28by%20ref%29))
  (bind (_isenemy _enemystats) (CallFunction|GetEnemyUnitStats OtherActor))
  (if (not (Utilities|Array|ContainsItem (Variables|Default|GetDamagedActors) OtherActor))
    (if _isenemy
      (if (CallFunction|IsEnemy (Default|GetAlignment _enemystats) (Variables|Default|GetAlignment))
        (Default|OnEnemyHit (Variables|Default|GetSpellController) (.AsCharacter (Utilities|Casting|CastToCharacter OtherActor)) _enemystats)
        (Utilities|Array|AddUnique (Variables|Default|GetDamagedActors) OtherActor)))))

(event EventBeginPlay
  (Utilities|FlowControl|DelayUntilNextTick)
  (Actor|DestroyActor))

(event Collision|EventActorBeginOverlap
  (params (OtherActor :type Actor%20Object%20Reference)))

(event EventTick
  (params (DeltaSeconds :type Float%20%28single-precision%29)))

(fn ConstructionScript)