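; Spell controller component for Spirit Slash, a player ability that attacks with an ephemeral sword.
; Cast start attaches a sword actor to the main-hand socket and undissolves it; cast end dissolves and destroys it.
; At the cast point it spawns a player-aligned hitbox aimed at the mouse, passing itself as controller.
; OnEnemyHit deals weapon-scaled damage from GetDamage, which also feeds the tooltip description.
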(event EventOnActiveSpellCastPoint
  (Game|SpawnActorfromClass "/Game/Abilities/SpiritSlash/BP_SpiritSlashHitbox.BP_SpiritSlashHitbox_C" (Math|Transform|MakeTransform (Transformation|GetActorLocation (Variables|Default|GetPlayerPawn)) (Math|Rotator|MakeRotfromX (Math|Vector|GetUnitDirection(Vector) (Transformation|GetActorLocation (Variables|Default|GetPlayerPawn)) (CallFunction|GetMouseWorldPosition (Variables|Default|GetPlayerPawn))))) "Undefined" 0 (Default|GetAlignment (Variables|/Game/Characters/PlayerDruid/BP_Player.BP_Player_C|GetUnitStatsComponent (Variables|Default|GetPlayerPawn))) self 0))

(event EventOnCastStarted
  (bind _returnvalue (Game|SpawnActorfromClass "/Game/Abilities/SpiritSlash/BP_SpiritSlashSword.BP_SpiritSlashSword_C" (Math|Transform|MakeTransform "0, 0, 0" "180.000000,90.000000, 0") "Undefined" 0 0))
  (Variables|Default|SetSwordActor _returnvalue)
  (Default|UndissolveAllMeshes (Variables|/Game/Abilities/SpiritSlash/BP_SpiritSlashSword.BP_SpiritSlashSword_C|GetReusableDissolveAgent _returnvalue) 1.0)
  (Transformation|AttachComponentToComponent (Variables|Default|GetSwordActor) (Variables|/Script/Engine.Character|GetMesh (Variables|Default|GetPlayerPawn)) "MainHandSocket" "SnapToTarget" "KeepRelative" "SnapToTarget" true))

(event EventOnCastEnded
  (Default|DissolveAllMeshesandDestroy (Variables|/Game/Abilities/SpiritSlash/BP_SpiritSlashSword.BP_SpiritSlashSword_C|GetReusableDissolveAgent (Variables|Default|GetSwordActor)) 1.0))

(fn OnEnemyHit
  (params (EnemyCharacter :type Character%20Object%20Reference) (EnemyStats :type Enemy%20Unit%20Stats%20Component%20Object%20Reference))
  (bind (_damage _weaponscaling _damagetype) (CallFunction|GetDamage))
  (Default|DealDamage EnemyStats (CallFunction|GetPlayerAbilityDI _damage _weaponscaling _damagetype "NewEnumerator0" self)))

(fn GetDamage
  (return 75.0 1.0 "NewEnumerator1"))

(fn GetDescriptionFields
  (return (Utilities|Struct|MakeS_SpellDescriptionFields "Spirit Slash" "Attack your enemies with an ephemeral blade that feels just like a proper melee weapon!" (Utilities|Array|MakeArray (Utilities|Struct|MakeS_SpellDescriptionFieldEntry "Base Damage" (Utilities|String|ToString(Float) (.Damage (CallFunction|GetDamage))) "NewEnumerator1")))))