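; BP_RockThrowProjectileImpactPhysics is a one-shot physics field actor for rock throw projectile impacts, breaking and scattering destructible geometry.
; On BeginPlay it applies external cluster strain through a linear radial falloff sized to its Sphere component.
; The same falloff culls two linear forces outside the sphere: a radial push from the center and a uniform push along the actor's forward vector.
; It destroys itself immediately afterwards.
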(event EventBeginPlay
  (bind _sphere (Variables|Default|GetSphere))
  (Class|FieldSystemComponent|ApplyPhysicsField (Variables|Field|GetFieldSystemComponent) true "Field_ExternalClusterStrain" 0 (Field|SetRadialFalloff (Variables|Default|GetRadialFalloff) 1e+10 0.0 1.0 0.0 (Components|Sphere|GetScaledSphereRadius _sphere) (Transformation|GetWorldLocation _sphere) "Field_Falloff_Linear"))
  (Class|FieldSystemComponent|ApplyPhysicsField (Variables|Field|GetFieldSystemComponent) true "Field_LinearForce" 0 (Field|SetCullingField (Variables|Default|GetCullingField) (Variables|Default|GetRadialFalloff) (Field|SetRadialVector (Variables|Default|GetRadialVector) 3e+03 (Transformation|GetWorldLocation (Variables|Default|GetSphere))) "Field_Culling_Outside"))
  (Class|FieldSystemComponent|ApplyPhysicsField (Variables|Field|GetFieldSystemComponent) true "Field_LinearForce" 0 (Field|SetCullingField (Variables|Default|GetCullingField) (Variables|Default|GetRadialFalloff) (Field|SetUniformVector (Variables|Default|GetUniformVector) 5e+03 (Math|Rotator|GetRotationXVector (Transformation|GetActorRotation))) "Field_Culling_Outside"))
  (Actor|DestroyActor))

(fn ConstructionScript)