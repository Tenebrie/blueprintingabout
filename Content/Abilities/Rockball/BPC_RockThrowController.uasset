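; Spell controller component for the Rock Throw ability, which hurls a rock projectile from its owner toward the mouse cursor's world position.
; On reaching the active cast point, it launches BP_RockThrowProjectile using the owner's alignment from its unit stats.
; Overrides supply a fixed cooldown and the spell's name and description text for display.
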(event EventOnActiveSpellCastPoint
  (bind _returnvalue (Components|GetOwner))
  (CallFunction|LaunchProjectileatPoint "/Game/Abilities/Rockball/BP_RockThrowProjectile.BP_RockThrowProjectile_C" (Transformation|GetActorLocation _returnvalue) (CallFunction|GetMouseWorldPosition (Components|GetOwner)) (Default|GetAlignment (.UnitStats (CallFunction|GetActorUnitStats _returnvalue))) "NewEnumerator1"))

(fn GetActiveSpellCooldown
  (return 3.0))

(fn GetDescriptionFields
  (return (Utilities|Struct|MakeS_SpellDescriptionFields "Rock Throw" "This spell is good to toss at things you want to sent flying.")))