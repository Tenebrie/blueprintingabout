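; Rock throw ability projectile, a child of a projectile base class that supplies the state and tick logic.
; On one state change, apparently impact, it destroys its sphere and spawns debris and impact physics actors at its transform, removing the debris after a delay.
; GetDamage returns fixed damage, weapon scaling and damage type regardless of target; Tick adds nothing beyond the parent call.
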(event EventTick
  (params (DeltaSeconds :type Float%20%28single-precision%29))
  (|CallParentFunction DeltaSeconds)
  (if (Utilities|Enum|Equal(Enum) (Variables|Default|GetProjectileState) "NewEnumerator2")
    _))

(event EventOnStateChanged
  (params (State :type E_ProjectileState%20Enum :default "NewEnumerator0"))
  (if (Utilities|Enum|Equal(Enum) State "NewEnumerator2")
    (Components|DestroyComponent (Variables|Default|GetSphere))
    (bind _returnvalue (Game|SpawnActorfromClass "/Game/Abilities/Rockball/BP_RockThrowProjectileDebris.BP_RockThrowProjectileDebris_C" (Transformation|GetActorTransform) "Undefined" 0 0))
    (Game|SpawnActorfromClass "/Game/Abilities/Rockball/BP_RockThrowProjectileImpactPhysics.BP_RockThrowProjectileImpactPhysics_C" (Transformation|GetActorTransform) "Undefined" 0 0)
    (Utilities|FlowControl|Delay 5.0)
    (Actor|DestroyActor _returnvalue)))

(fn ConstructionScript
  (|CallParentFunction))

(fn GetDamage
  (params (DamageImpactTarget :type Actor%20Object%20Reference))
  (return 1e+02 0.5 "NewEnumerator1"))