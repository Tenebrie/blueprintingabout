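; Ability controller for the Magic Fountain spell, handling its cast as an active spell.
; On cast, it starts the player controller's global cooldown and spawns a Magic Fountain projectile, passing itself as the projectile's controller.
; The spawn point is a short, fixed distance from the controlled pawn in a random horizontal direction, found by rotating a unit vector around the Z axis.
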(event EventOnSpellCastasActive
  (Default|StartGlobalCooldown (Variables|Default|GetPlayerController) 1.0)
  (Game|SpawnActorfromClass "/Game/Abilities/MagicFountain/BP_MagicFouintainProjectile.BP_MagicFouintainProjectile_C" (Math|Conversions|ToTransform(Vector) (+ (Transformation|GetActorLocation (Pawn|GetControlledPawn (Variables|Default|GetPlayerController))) (* (Math|Vector|RotateVectorAroundAxis (Math|Vector|MakeVector 1.0 0.0 0.0) (Math|Random|RandomFloatinRange 0.0 3.6e+02) "0, 0,1.000000") 5e+01))) "Undefined" 0 self "NewEnumerator0" 0))