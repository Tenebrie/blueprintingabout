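; Spell slot component that holds one assigned spell for an input binding, active or passive, and manages its casting and cooldowns.
; Assignment adds the spell's controller component to the player pawn, and a pawn change recreates it on the new pawn.
; OnValidatedTick checks cooldowns, spends mana, starts global and spell cooldowns, then triggers the controller's cast point.
; Tick counts both cooldowns down to the hotbar widget, while assignment changes refresh hotbar and inventory icons.
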(event Custom|OnValidatedTick
  (if (CallFunction|IsSlotOffCooldown)
    (bind _success (Default|ConsumeMana (Variables|/Game/Characters/PlayerDruid/BP_Player.BP_Player_C|GetUnitStatsComponent (Variables|Default|GetPlayerPawn)) (Default|GetManaCost (Variables|AssignedSpell|GetAssignedSpellController))))
    (if _success
      (Default|StartGlobalCooldown (Variables|Provided|GetPlayerController) (.Duration (CallFunction|GetCastAnimationTimings (.Animation (Utilities|Struct|BreakS_Spell (Variables|AssignedSpell|GetAssignedSpellData))) (Default|GetCurrentCastSpeed (.AsPC%20Player%20Controller (Utilities|Casting|CastToPC_PlayerController (Pawn|GetController (Variables|Default|GetPlayerPawn))))))))
      (CallFunction|StartSpellCooldown (Default|GetSpellCooldown (Variables|AssignedSpell|GetAssignedSpellController)))
      (Default|OnActiveSpellCastPoint (Variables|AssignedSpell|GetAssignedSpellController)))))

(event EventTick
  (params (DeltaSeconds :type Float%20%28single-precision%29))
  (Variables|Default|SetDeltaSeconds DeltaSeconds)
  (Variables|SpellCooldown|SetRemainingSpellCooldown (Math|Float|Max(Float) (- (Variables|SpellCooldown|GetRemainingSpellCooldown) (Variables|Default|GetDeltaSeconds)) 0.0))
  (Variables|SpellCooldown|SetRemainingGlobalCooldown (Math|Float|Max(Float) (- (Variables|SpellCooldown|GetRemainingGlobalCooldown) (Variables|Default|GetDeltaSeconds)) 0.0))
  (CallFunction|UpdateHotbarCooldown))

(event EventBeginPlay
  (bind _asbp_player (Utilities|Casting|CastToBP_Player (Pawn|GetControlledPawn (Variables|Provided|GetPlayerController))))
  (Variables|Default|SetPlayerPawn _asbp_player)
  (CallFunction|InferBindingType)
  (bind _bindinginputtext (CallFunction|GetBindingFriendlyText))
  (Variables|Default|SetBindingFriendlyText _bindinginputtext))

(fn AssignSpell
  (params (SpellData :type S%20Spell%20Structure))
  (CallFunction|UnassignSpell)
  (bind _output_get (Variables|AssignedSpell|SetAssignedSpellData SpellData))
  (bind _returnvalue (Game|AddComponentbyClass (Variables|Default|GetPlayerPawn) (.ControlComponentClass (Utilities|Struct|BreakS_Spell _output_get)) self))
  (Variables|AssignedSpell|SetAssignedSpellController _returnvalue)
  (CallFunction|UpdateUI))

(fn UnassignSpell
  (if (Utilities|IsValid (Variables|AssignedSpell|GetAssignedSpellController))
    (Components|DestroyComponent (Variables|AssignedSpell|GetAssignedSpellController))
    (Variables|AssignedSpell|SetAssignedSpellData "")
    (Variables|AssignedSpell|SetAssignedSpellController 0)
    (CallFunction|UpdateUI)))

(fn IsSpellAssigned
  (return (Utilities|IsValid (Variables|AssignedSpell|GetAssignedSpellController))))

(fn RegisterHotbarWidget
  (params (HotbarWidget :type UI%20Spell%20Slot%20Hotbar%20Item%20Object%20Reference))
  (Variables|Default|SetHotbarWidget HotbarWidget))

(fn RegisterInventoryWidget
  (params (InventoryWidget :type UI%20Spell%20Slot%20Grid%20Item%20Object%20Reference))
  (Variables|Default|SetInventoryWidget InventoryWidget))

(fn GetBindingFriendlyText
  (switch Utilities|FlowControl|Switch|SwitchonE_SpellSlotBindingType (Variables|Default|GetBindingType)
    (:NewEnumerator0
      (switch Utilities|FlowControl|Switch|SwitchonE_SpellSlotBinding (Variables|Provided|GetBinding)
        (:NewEnumerator0
          (return "LMB"))
        (:NewEnumerator1
          (return "RMB"))
        (:NewEnumerator3
          (return "Shift"))))
    (:NewEnumerator1
      (return "Passive"))))

(fn InferBindingType
  (if (Math|Boolean|ORBoolean (Utilities|Enum|Equal(Enum) (Variables|Provided|GetBinding) "NewEnumerator0") (Utilities|Enum|Equal(Enum) (Variables|Provided|GetBinding) "NewEnumerator1") (Utilities|Enum|Equal(Enum) (Variables|Provided|GetBinding) "NewEnumerator3"))
    (Variables|Default|SetBindingType "NewEnumerator0")
    (else
      (Variables|Default|SetBindingType "NewEnumerator1"))))

(fn UpdateUI
  (bind _inventorywidget (Variables|Default|GetInventoryWidget))
  (Utilities|FlowControl|Sequence
    (:then_0
      ;[1 1 1] Inventory
      (if (Utilities|IsValid _inventorywidget)
        (Default|UpdateIconVisibility _inventorywidget)))
    (:then_1
      ;[1 1 1] Hotbar
      (if (Utilities|IsValid (Variables|Default|GetHotbarWidget))
        (Default|UpdateIconVisibility (Variables|Default|GetHotbarWidget))))))

(fn UpdateHotbarCooldown
  (if (Utilities|IsValid (Variables|Default|GetHotbarWidget))
    (Default|UpdateCooldownState (Variables|Default|GetHotbarWidget) (Variables|SpellCooldown|GetRemainingSpellCooldown) (Variables|SpellCooldown|GetMaximumSpellCooldown) (Variables|SpellCooldown|GetRemainingGlobalCooldown) (Variables|SpellCooldown|GetMaximumGlobalCooldown))))

(fn StartSpellCooldown
  (params (Time :type Float%20%28double-precision%29))
  (bind _output_get (Variables|SpellCooldown|SetRemainingSpellCooldown Time))
  (Variables|SpellCooldown|SetMaximumSpellCooldown _output_get)
  (CallFunction|UpdateHotbarCooldown))

(fn StartGlobalCooldownonThisSlot
  (params (Time :type Float%20%28double-precision%29))
  (bind _output_get (Variables|SpellCooldown|SetRemainingGlobalCooldown Time))
  (Variables|SpellCooldown|SetMaximumGlobalCooldown _output_get)
  (CallFunction|UpdateHotbarCooldown))

(fn IsSlotOffCooldown
  (return (and (<= (Variables|SpellCooldown|GetRemainingSpellCooldown) 0.0) (<= (Variables|SpellCooldown|GetRemainingGlobalCooldown) 0.0))))

(fn UpdatePawn
  (params (NewPawn :type BP%20Player%20Object%20Reference))
  (if (Utilities|IsValid (Variables|AssignedSpell|GetAssignedSpellController))
    (LocalVariables|SetSpellData (Variables|AssignedSpell|GetAssignedSpellData))
    (CallFunction|UnassignSpell)
    (Variables|Default|SetPlayerPawn NewPawn)
    (CallFunction|AssignSpell (LocalVariables|GetSpellData))
    (else
      (Variables|Default|SetPlayerPawn NewPawn))))

(fn CanTransitionIntoSlot
  (if (Utilities|IsValid (Variables|AssignedSpell|GetAssignedSpellController))
    (return (and (<= (Variables|SpellCooldown|GetRemainingSpellCooldown) 0.0) (>= (.CurrentMana (Default|GetMana (.UnitStats (CallFunction|GetActorUnitStats (Variables|Default|GetPlayerPawn))))) (Default|GetManaCost (Variables|AssignedSpell|GetAssignedSpellController)))))
    (else
      (return false))))