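; BPC_IgniteBuff is a stackable burn buff component in the Fireball ability folder that deals damage over time to its owning actor.
; Added stacks grow a pool of remaining damage, refresh the duration and re-spread that pool over the base duration as damage per second.
; Tick is throttled by ticks per second, sending time-scaled damage to the owner's UnitStats and subtracting it from the pool.
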(event EventBeginPlay)

(event EventTick
  (params (DeltaSeconds :type Float%20%28single-precision%29))
  (|CallParentFunction DeltaSeconds)
  (bind (_shouldcontinue _deltatime) (CallFunction|ThrottleTick 1.0 DeltaSeconds (Variables|Default|GetThrottle%20Tick%20State)))
  (if _shouldcontinue
    (Default|DealDamage (.UnitStats (CallFunction|GetActorUnitStats (Components|GetOwner))) (CallFunction|GetBurnDI (* _deltatime (Variables|Default|GetDamagePerSecond)) "NewEnumerator2"))
    (Variables|Default|SetDamageToDeal (- (Variables|Default|GetDamageToDeal) (* _deltatime (Variables|Default|GetDamagePerSecond))))))

(fn OnExtraStacksAdded
  (params (StackCount :type Integer))
  (bind _output_get (Variables|Default|SetDamageToDeal (+ (Variables|Default|GetDamageToDeal) (* StackCount (CallFunction|GetDamagePerStack)))))
  (CallFunction|RefreshDuration)
  (Variables|Default|SetDamagePerSecond (/ _output_get (Variables|Default|GetBaseDuration))))

(fn GetDamagePerStack
  (return 9.0))