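; Fireball projectile whose speed, damage and steering are modified by runes.
; Speed runes raise initial speed at construction; Fatal Acceleration increases speed each tick and adds speed-scaled bonus damage to the base.
; Magnetic steering periodically picks the closest enemy unit within a frontal cone and range, then yaws toward it, scaled by proximity and angle.
; That steering is gated by the Fatal Acceleration flag, not a separate Magnetic one.
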(event Custom|OnTickFatalAcceleration
  (Variables|Default|SetProjectileSpeed (+ (Math|Float|SelectFloat (* (Variables|Default|GetDeltaSeconds) (Variables|FatalAccelerationRune|GetFireballAcceleration)) 0.0 (Variables|FatalAccelerationRune|GetFireballFatalAccelerationRuneEnabled)) (Variables|Default|GetProjectileSpeed))))

(event Custom|OnTickMagneticRune
  (Utilities|FlowControl|Sequence
    (:then_0
      (Variables|MagneticRune|SetMagneticRuneSinceUpdate (+ (Variables|MagneticRune|GetMagneticRuneSinceUpdate) (Variables|Default|GetDeltaSeconds)))
      (if (> (Variables|MagneticRune|GetMagneticRuneSinceUpdate) 0.2)
        (Variables|MagneticRune|SetMagneticRuneSinceUpdate 0.0)
        (bind _outactors (Actor|GetAllActorswithTag (CallFunction|GetTagbyValue "(TagName=\"is_unit\")")))
        (bind _output (CallFunction|GetActorsWithinFrontalAngle _outactors))
        (bind _closestenemy (CallFunction|GetClosestEnemytoActor self _output (Variables|Default|GetProjectileAlignment) 4e+02))
        (Variables|MagneticRune|SetClosestEnemy _closestenemy)))
    (:then_1
      (if (and (Variables|FatalAccelerationRune|GetFireballFatalAccelerationRuneEnabled) (Utilities|IsValid (Variables|MagneticRune|GetClosestEnemy)))
        (Transformation|AddActorLocalRotation (Math|Rotator|MakeRotator 0.0 0.0 (* (* (Math|Float|Sign(Float) (* (CallFunction|GetAngleBetweenVectors (Math|Vector|GetUnitDirection(Vector) (Transformation|GetActorLocation) (Transformation|GetActorLocation (Variables|MagneticRune|GetClosestEnemy))) (Math|Vector|GetForwardVector (Transformation|GetActorRotation))) 1.0)) -1.0) (Math|Float|Min(Float) (Math|Float|Absolute(Float) (* (CallFunction|GetAngleBetweenVectors (Math|Vector|GetUnitDirection(Vector) (Transformation|GetActorLocation) (Transformation|GetActorLocation (Variables|MagneticRune|GetClosestEnemy))) (Math|Vector|GetForwardVector (Transformation|GetActorRotation))) 1.0)) (* (+ (Math|Float|Power (Math|Float|MapRangeClamped (Transformation|GetDistanceTo (Variables|MagneticRune|GetClosestEnemy)) 3e+02 5e+01 0.0 (Variables|MagneticRune|GetRotationSpeed)) 4.0) (Math|Float|Absolute(Float) (CallFunction|GetAngleBetweenVectors (Math|Vector|GetUnitDirection(Vector) (Transformation|GetActorLocation) (Transformation|GetActorLocation (Variables|MagneticRune|GetClosestEnemy))) (Math|Vector|GetForwardVector (Transformation|GetActorRotation))))) (Variables|Default|GetDeltaSeconds))))) false false)))))

(event EventTick
  (params (DeltaSeconds :type Float%20%28single-precision%29))
  (|CallParentFunction DeltaSeconds)
  (CallFunction|OnTickFatalAcceleration)
  (CallFunction|OnTickMagneticRune))

(fn ConstructionScript
  (|CallParentFunction)
  (Variables|Default|SetProjectileSpeed (+ (Variables|Default|GetProjectileSpeed) (* (Variables|SpeedRune|GetFireballSpeedRuneCount) (Variables|SpeedRune|GetProjectileSpeedPerRune)))))

(fn GetDamage
  (return (+ (Math|Float|SelectFloat (/ (Variables|Default|GetProjectileSpeed) 1e+02) 0.0 (Variables|FatalAccelerationRune|GetFireballFatalAccelerationRuneEnabled)) 25.0)))

(fn GetActorsWithinFrontalAngle
  (params (Actors :type Array%20of%20Actor%20Object%20References))
  (LocalVariables|SetAnswer (Utilities|Array|MakeArray))
  (for _array_element Actors
    (if (< (Math|Float|Absolute(Float) (CallFunction|GetAngleBetweenVectors (Math|Vector|GetUnitDirection(Vector) (Transformation|GetActorLocation) (Transformation|GetActorLocation _array_element)) (Math|Vector|GetForwardVector (Transformation|GetActorRotation)))) 45.0)
      (Utilities|Array|Add (LocalVariables|GetAnswer) _array_element)))
  (return (LocalVariables|GetAnswer)))