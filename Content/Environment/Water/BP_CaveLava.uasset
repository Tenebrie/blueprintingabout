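; Cave lava hazard that periodically damages units standing in it.
; Collider overlap events maintain a list of submersed actors.
; Tick is throttled to run twice a second, dealing a fixed damage instance to every listed actor that has unit stats.
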(event OnComponentBeginOverlap(Collider)
  (params (OverlappedComponent :type Primitive%20Component%20Object%20Reference) (OtherActor :type Actor%20Object%20Reference) (OtherComp :type Primitive%20Component%20Object%20Reference) (OtherBodyIndex :type Integer) (bFromSweep :type Boolean) (SweepResult :type Hit%20Result%20Structure%20%28by%20ref%29))
  (Utilities|Array|Add (Variables|Default|GetSubmersedActors) OtherActor))

(event OnComponentEndOverlap(Collider)
  (params (OverlappedComponent :type Primitive%20Component%20Object%20Reference) (OtherActor :type Actor%20Object%20Reference) (OtherComp :type Primitive%20Component%20Object%20Reference) (OtherBodyIndex :type Integer))
  (Utilities|Array|RemoveItem (Variables|Default|GetSubmersedActors) OtherActor))

(event EventBeginPlay)

(event Collision|EventActorBeginOverlap
  (params (OtherActor :type Actor%20Object%20Reference)))

(event EventTick
  (params (DeltaSeconds :type Float%20%28single-precision%29))
  (bind _shouldcontinue (CallFunction|ThrottleTick 2.0 DeltaSeconds (Variables|Default|GetThrottle%20Tick%20State)))
  (if _shouldcontinue
    (for _array_element (Variables|Default|GetSubmersedActors)
      (if (.IsUnit (CallFunction|GetActorUnitStats _array_element))
        (Default|DealDamage (.UnitStats (CallFunction|GetActorUnitStats _array_element)) (Utilities|Struct|MakeS_DamageInstance 25.0 "NewEnumerator0" "NewEnumerator0"))))))

(fn ConstructionScript)