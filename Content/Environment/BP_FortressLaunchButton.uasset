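; Reusable fortress launch button that populates battle fortress spawn points with trolls when interacted with.
; HoverInfoAgent's OnInteract loops over every BP_BattleFortressSpawn, randomly spawning a BP_TrollEnemy, a more common BP_HordeTrollEnemy, or nothing just above it.
; Each troll is possessed by a newly spawned AIController, targets the interactor through AggroPawn and takes its level from that player's PlayerProgressionComponent.
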(event OnInteract(HoverInfoAgent)
  (params (Interactor :type Pawn%20Object%20Reference))
  (bind _outactors (Actor|GetAllActorsOfClass "/Game/Environment/BP_BattleFortressSpawn.BP_BattleFortressSpawn_C"))
  (for _array_element _outactors
    (if (< (Math|Random|RandomFloatinRange 0.0 1.0) 0.1)
      (bind _returnvalue (Game|SpawnActorfromClass "/Game/Characters/Enemies/Trolls/BP_TrollEnemy.BP_TrollEnemy_C" (Math|Conversions|ToTransform(Vector) (+ (Transformation|GetActorLocation _array_element) "0,0,50.000000")) "Undefined" 0 0))
      (bind _returnvalue_2 (Game|SpawnActorfromClass "/Script/AIModule.AIController" (Math|Transform|MakeTransform "0, 0, 0") "Undefined" 0 0))
      (if (Utilities|IsValid _returnvalue)
        (Pawn|Possess _returnvalue_2 _returnvalue)
        (Variables|/Game/Characters/Enemies/BP_NewBaseEnemy.BP_NewBaseEnemy_C|SetAggroPawn _returnvalue Interactor)
        (bind _asps_player_state (Utilities|Casting|CastToPS_PlayerState (Variables|/Script/Engine.Controller|GetPlayerState (Pawn|GetController Interactor))))
        (Default|SetCurrentLevel (Variables|/Game/Characters/Enemies/BP_NewBaseEnemy.BP_NewBaseEnemy_C|GetEnemyStatsComponent _returnvalue) (Variables|/Game/Characters/PlayerDruid/BPC_PlayerProgression.BPC_PlayerProgression_C|GetCurrentLevel (Variables|/Game/Characters/PlayerDruid/PS_PlayerState.PS_PlayerState_C|GetPlayerProgressionComponent _asps_player_state))))
      (elif (< (Math|Random|RandomFloatinRange 0.0 1.0) 0.3)
        (bind _returnvalue_3 (Game|SpawnActorfromClass "/Game/Characters/Enemies/Trolls/BP_HordeTrollEnemy.BP_HordeTrollEnemy_C" (Math|Conversions|ToTransform(Vector) (+ (Transformation|GetActorLocation _array_element) "0,0,50.000000")) "Undefined" 0 0))
        (bind _returnvalue_4 (Game|SpawnActorfromClass "/Script/AIModule.AIController" (Math|Transform|MakeTransform "0, 0, 0") "Undefined" 0 0))
        (if (Utilities|IsValid _returnvalue_3)
          (Pawn|Possess _returnvalue_4 _returnvalue_3)
          (Variables|/Game/Characters/Enemies/BP_NewBaseEnemy.BP_NewBaseEnemy_C|SetAggroPawn _returnvalue_3 Interactor)
          (bind _asps_player_state_2 (Utilities|Casting|CastToPS_PlayerState (Variables|/Script/Engine.Controller|GetPlayerState (Pawn|GetController Interactor))))
          (Default|SetCurrentLevel (Variables|/Game/Characters/Enemies/BP_NewBaseEnemy.BP_NewBaseEnemy_C|GetEnemyStatsComponent _returnvalue_3) (Variables|/Game/Characters/PlayerDruid/BPC_PlayerProgression.BPC_PlayerProgression_C|GetCurrentLevel (Variables|/Game/Characters/PlayerDruid/PS_PlayerState.PS_PlayerState_C|GetPlayerProgressionComponent _asps_player_state_2))))))))

(event EventBeginPlay)

(event Collision|EventActorBeginOverlap
  (params (OtherActor :type Actor%20Object%20Reference)))

(event EventTick
  (params (DeltaSeconds :type Float%20%28single-precision%29)))

(fn ConstructionScript)

(fn IsSingleUse
  (return false))