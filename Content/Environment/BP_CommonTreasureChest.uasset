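; A common treasure chest prop that opens once when interacted with but grants no real loot yet.
; The hover agent's interact event sets an opened flag and shows a random joke message as floating text on the interactor.
; While opened, Tick rotates the lid open at a constant, frame-rate-independent speed until it passes its roll limit.
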(event OnInteract(HoverInfoAgent)
  (params (Interactor :type Pawn%20Object%20Reference))
  (if (not (Variables|Default|GetIsOpened))
    (Variables|Default|SetIsOpened true)
    (Default|CreateFloatingInfoText (Variables|Default|GetFloatingTextCreator) Interactor (Utilities|Select :Index (Math|Random|RandomIntegerinRange 0 11) :Option%200 "You got imaginary loot!" :Option%201 "You just got chest'ed!" :Option%202 "This was not a mimic! ...or was it?" :Option%203 "Sorry, your loot is in another castle." :Option%204 "Nope." :Option%205 "I swear the loot was just here!" :Option%206 "This chest will be full in a future version." :Option%207 "No loot here. Sorry." :Option%208 "I really wish I had loot ready by now, but alas." :Option%209 "You got an imaginary weapon!" :Option%2010 "You got an imaginary armor piece!" :Option%2011 "YOU GOT AN IMAGINARY LEGENDARY.") "(R=1.000000,G=0.298269,B=0.000000,A=1.000000)")))

(event EventTick
  (params (DeltaSeconds :type Float%20%28single-precision%29))
  (if (and (Variables|Default|GetIsOpened) (> (.Roll (Math|Rotator|BreakRotator (Transformation|GetWorldRotation (Variables|Default|GetSM_Prop_Chest_Wood_Lid)))) -135.0))
    (Transformation|AddLocalRotation (Variables|Default|GetSM_Prop_Chest_Wood_Lid) (Math|Rotator|MakeRotator (* DeltaSeconds -135.0) 0.0 0.0) false false)))

(fn ConstructionScript)