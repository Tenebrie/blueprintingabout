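; An interactable button that generates a test rift by streaming in a grid of tile level instances.
; On HoverInfoAgent interaction, it calls GenerateRift at a fixed offset from the button's location.
; GenerateRift loops over a hard-coded square grid, and each point loads the same RiftTileTest level at its spaced position.
; IsSingleUse returns false, and nothing clears previously loaded tiles.
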(event OnInteract(HoverInfoAgent)
  (params (Interactor :type Pawn%20Object%20Reference))
  (CallFunction|GenerateRift (+ (Transformation|GetActorLocation) "0.000000,550.000000,-100.000000")))

(fn ConstructionScript)

(fn GenerateRift
  (params (RiftPosition :type Vector))
  (LocalVariables|SetGridSize 1e+03)
  (LocalVariables|SetGridSlotsX 3)
  (LocalVariables|SetGridSlotsY 3)
  (for _index (range 0 (- (LocalVariables|GetGridSlotsX) 1))
    (for _index_2 (range 0 (- (LocalVariables|GetGridSlotsY) 1))
      (CallFunction|GenerateRiftGridPoint RiftPosition _index _index_2 (LocalVariables|GetGridSize)))))

(fn GenerateRiftGridPoint
  (params (RiftPosition :type Vector) (GridX :type Integer) (GridY :type Integer) (GridSize :type Float%20%28double-precision%29))
  (Class|LevelStreamingDynamic|LoadLevelInstancebySoftObjectPtr "/Game/Maps/RiftTiles/RiftTileTest.RiftTileTest" (+ RiftPosition (Math|Vector|MakeVector (* (Math|Conversions|ToFloat(Integer) GridX) GridSize) (* (Math|Conversions|ToFloat(Integer) GridY) GridSize) 0.0)) "0, 0, 0" "" 0 false))

(fn IsSingleUse
  (return false))